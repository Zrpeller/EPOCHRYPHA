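; Turret Blueprint that targets the closest visible pawn within sensing range and fires projectile bursts at it.
; Each tick it picks a target by sphere overlap and line-of-sight test, then turns its capsule toward it at constant speed with pitch locked level.
; Once the fire cooldown passes and a dot product confirms aim, a delayed DoN loop spawns three TestProjectiles from the gun's Muzzle socket.
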(event `self.ReceiveTick`
  (params (DeltaSeconds :type "Float (single-precision)"))
  (`self.FindBestTarget`)
  (`self.Target`
    (:`then`
      (`self.UpdateEnemyRotation` DeltaSeconds)
      (`self.UpdateFire`))
    (:`else`)))

(event `Fire`
  (set `self.LastFireTime` (`KismetSystemLibrary.GetGameTimeInSeconds`))
  (`|ExecutionSequence`
    (:`then_0`
      (goto _label :!via `Reset`))
    (:`then_1`
      (`/Engine/EditorBlueprintResources/StandardMacros.Do N` 3 :!label _label
        (:`Exit`
          (`|SpawnActorFromClass` "/Game/NewRanged/TestProjectile.TestProjectile_C" (`SceneComponent.GetSocketTransform` (`self.Gun`) "Muzzle" "RTS_World") "Undefined" "OverrideRootScale" null null)
          (`KismetSystemLibrary.Delay` 0.2)
          (goto _label))))))

(fn `FindBestTarget`
  (locals (`BestDistance (Local)` :type "Float (double-precision)") (`CurrentDistance (Local)` :type "Float (double-precision)") (`BestTarget (Local)` :type "Actor Object Reference") (`CurrentTarget (Local)` :type "Actor Object Reference"))
  (set `local.BestDistance (Local)` (+ (`self.SensingRange`) 1.0))
  (bind _outactors (`KismetSystemLibrary.SphereOverlapActors` (`self.K2_GetActorLocation`) (`self.SensingRange`) (`|MakeArray` "ObjectTypeQuery3" :!type "EObjectTypeQuery Enum")))
  (for _array_element _outactors
    (bind _output_get (set `local.CurrentTarget (Local)` _array_element))
    (bind _output_get_2 (set `local.CurrentDistance (Local)` (`self.GetDistanceTo` _output_get self)))
    (if (or (< _output_get_2 (`local.BestDistance (Local)`)) (not (`KismetSystemLibrary.IsValid` (`local.BestTarget (Local)`))))
      (bind _result (`/Game/NewRanged/MyFunctionLibrary.HasLineOfSight` (`SceneComponent.K2_GetComponentLocation` (`self.CapsuleComponent`)) (`self.K2_GetActorLocation` (`local.CurrentTarget (Local)`)) (`|MakeArray` self (`local.CurrentTarget (Local)`) :!type "Actor Object Reference")))
      (if _result
        (set `local.BestTarget (Local)` (`local.CurrentTarget (Local)`))
        (set `local.BestDistance (Local)` (`local.CurrentDistance (Local)`)))))
  (set `self.Target` (`local.BestTarget (Local)`)))

(fn `UpdateEnemyRotation`
  (params (DeltaSeconds :type "Float (double-precision)"))
  (locals (NewRotation :type "Rotator Structure" :default (struct)))
  (bind _output_get (set `local.NewRotation` (`KismetMathLibrary.RInterpTo_Constant` (`SceneComponent.K2_GetComponentRotation` (`self.CapsuleComponent`)) (`KismetMathLibrary.FindLookAtRotation` (`SceneComponent.K2_GetComponentLocation` (`self.CapsuleComponent`)) (`self.K2_GetActorLocation` (`self.Target`))) (`local.DeltaSeconds`) (`self.RotationSpeed`))))
  (`SceneComponent.K2_SetWorldRotation` (`self.CapsuleComponent`) (`KismetMathLibrary.MakeRotator` (.roll _output_get) (`KismetMathLibrary.ClampAngle` (.pitch _output_get)) (.yaw _output_get)) false false))

(fn `UpdateFire`
  (if (> (- (`KismetSystemLibrary.GetGameTimeInSeconds`) (`self.LastFireTime`)) (`self.FireRate`))
    (if (> (`KismetMathLibrary.Dot_VectorVector` (`KismetMathLibrary.GetDirectionUnitVector` (`SceneComponent.K2_GetComponentLocation` (`self.CapsuleComponent`)) (`self.K2_GetActorLocation` (`self.Target`))) (`SceneComponent.GetForwardVector` (`self.CapsuleComponent`))) 0.99)
      (`self.Fire`))))

(fn `UserConstructionScript`)