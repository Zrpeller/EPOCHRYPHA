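; Fluid Flux modifier actor that wraps a Gerstner wave modifier component for the water simulation.
; Construction runs the parent script, then adds a box component snapped to the Gerstner component's transform.
; It reports that it cannot render waves, while exposing the Gerstner component's material instance as its only wave texture material.
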(fn `CanRenderWave`
  (returns (CanRender :type Boolean))
  (return false))

(fn `GetWaveTextureMaterials`
  (returns (MaterialInstances :type "Array of MaterialInstanceDynamic Object Reference"))
  (return (`|MakeArray` (`/Game/Levels/LVL_Blockout_4_A/Water/FluidFlux/Simulation/Modifiers/Components/BP_FluxModifierWaveComponent.MaterialInstance` (`self.BP_FluxModifierGerstnerComponent`)))))

(fn `UserConstructionScript`
  (`parent.UserConstructionScript`)
  (bind _returnvalue (`AddComponent|NODE_AddBoxComponent-0` :`bManualAttachment` true))
  (`SceneComponent.K2_AttachToComponent` _returnvalue (`self.BP_FluxModifierGerstnerComponent`) "None" "SnapToTarget" "SnapToTarget" "SnapToTarget" true))