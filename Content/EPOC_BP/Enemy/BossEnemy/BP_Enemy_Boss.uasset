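; Boss enemy Blueprint that manages health, the boss health bar and death, ending in a win level.
; BeginPlay adds a health bar widget, fills health to max and caches the AI_Boss controller.
; AnyDamage subtracts health after a brief delay and updates the first found bar against a hardcoded maximum.
; At zero health it disables collision and movement, sets the blackboard's dead flag, then opens the win level after a pause.
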(event `self.ReceiveBeginPlay`
  (bind _returnvalue (`|CreateWidget` "/Game/EPOC_BP/Enemy/BossEnemy/WBP_BossHealthBar.WBP_BossHealthBar_C"))
  (bind _output_get (set `self.bossHealth` _returnvalue))
  (`UserWidget.AddToViewport` _output_get 0)
  (set `self.health` (`self.MaxHealth`))
  (bind _foundwidgets (`WidgetBlueprintLibrary.GetAllWidgetsOfClass` "/Game/EPOC_BP/Enemy/BossEnemy/WBP_BossHealthBar.WBP_BossHealthBar_C"))
  (set `self.bossHealthBars` _foundwidgets)
  (bind _asai_boss (cast `/Game/EPOC_BP/Enemy/BossEnemy/AI_Boss` (`self.GetController`)))
  (set `self.AsBossController` _asai_boss)
  (set `self.enemyHealth` 2)
  (cast `/Game/EPOC_BP/Enemy/BossEnemy/AI_Boss` (`self.AsBossController`)))

(event `self.ReceiveTick`
  (params (DeltaSeconds :type "Float (single-precision)")))

(event `self.ReceiveAnyDamage`
  (params (Damage :type "Float (single-precision)") (DamageType :type "DamageType Object Reference") (InstigatedBy :type "Controller Object Reference") (DamageCauser :type "Actor Object Reference"))
  (`KismetSystemLibrary.Delay` 0.05)
  (bind _output_get (set `self.health` (- (`self.health`) Damage)))
  (set `/Game/EPOC_BP/Enemy/BossEnemy/WBP_BossHealthBar.bossHealthPercent` (/ _output_get 3000.0) (`|GetArrayItem` (`self.bossHealthBars`)))
  (if (<= _output_get 0.0)
    (`PrimitiveComponent.SetCollisionEnabled` (`self.CapsuleComponent`) "NoCollision")
    (`CharacterMovementComponent.DisableMovement` (`self.CharacterMovement`))
    (set `self.Dying?` true)
    (`BlackboardComponent.SetValueAsBool` (`AIBlueprintHelperLibrary.GetBlackboard` (`self.AsBossController`)) "Dead?" true)
    (`KismetSystemLibrary.Delay` 3.0)
    (`GameplayStatics.OpenLevel` "BUILD_WinLevel")
    (`self.K2_DestroyActor`)))

(fn `UserConstructionScript`)