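; Support enemy character Blueprint that extends a parent class, setting its own health and movement speed on BeginPlay.
; Tick replays the caster death animation every frame while health is zero or below.
; DamageBox end overlap clears TouchingPlayer for the player unless dying, but begin overlap is empty.
; Attack logic (AI blackboard flag, hitbox spawning) is disconnected, as is the use of a local delayed-loop macro.
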(event `self.ReceiveTick`
  (params (DeltaSeconds :type "Float (single-precision)"))
  (if (<= (`self.health`) 0.0)
    (`SkeletalMeshComponent.PlayAnimation` (`self.Mesh`) "/Game/Character_Rigs/Caster_Enemy/Animations/Caster_Death_Retargeted.Caster_Death_Retargeted" false)))

(event `self.ReceiveBeginPlay`
  (`parent.ReceiveBeginPlay`)
  (set `self.health` 45.0)
  (set `self.MovementSpeed` 550.0))

(event `self.DamageBox.OnComponentBeginOverlap`
  (params (OverlappedComponent :type "PrimitiveComponent Object Reference") (OtherActor :type "Actor Object Reference") (OtherComp :type "PrimitiveComponent Object Reference") (OtherBodyIndex :type Integer) (bFromSweep :type Boolean) (SweepResult :type "HitResult Structure (by ref)")))

(event `self.DamageBox.OnComponentEndOverlap`
  (params (OverlappedComponent :type "PrimitiveComponent Object Reference") (OtherActor :type "Actor Object Reference") (OtherComp :type "PrimitiveComponent Object Reference") (OtherBodyIndex :type Integer))
  (if (not (`self.Dying?`))
    (cast `/Game/EPOC_BP/EPOC_CONTENT/Blueprints/PlayerBlueprints/BP_Player` OtherActor)
    (set `self.TouchingPlayer` false)))

(fn `UserConstructionScript`
  (`parent.UserConstructionScript`))