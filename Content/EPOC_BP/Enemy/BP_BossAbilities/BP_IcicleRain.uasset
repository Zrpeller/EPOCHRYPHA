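; BP_IcicleRain is a boss ability area hazard that damages players standing inside it and destroys itself four seconds after BeginPlay.
; Every Tick it queries the DmgArea component for overlapping BP_Player pawns and applies a small hit of DMG_SlowDamage to each.
; BeginPlay also caches all players in ActivePlayers, which the damage logic does not read, and the overlap events are empty.
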(event `self.ReceiveBeginPlay`
  (bind _outactors (`GameplayStatics.GetAllActorsOfClass` "/Game/EPOC_BP/EPOC_CONTENT/Blueprints/PlayerBlueprints/BP_Player.BP_Player_C"))
  (set `self.ActivePlayers` _outactors)
  (`KismetSystemLibrary.Delay` 4.0)
  (`self.K2_DestroyActor`))

(event `self.dmgArea.OnComponentBeginOverlap`
  (params (OverlappedComponent :type "PrimitiveComponent Object Reference") (OtherActor :type "Actor Object Reference") (OtherComp :type "PrimitiveComponent Object Reference") (OtherBodyIndex :type Integer) (bFromSweep :type Boolean) (SweepResult :type "HitResult Structure (by ref)")))

(event `self.ReceiveTick`
  (params (DeltaSeconds :type "Float (single-precision)"))
  (bind _dmgarea (`self.dmgArea`))
  (bind _outactors (`GameplayStatics.GetAllActorsOfClass` null))
  (bind _outactors_2 (`KismetSystemLibrary.ComponentOverlapActors` _dmgarea (`SceneComponent.K2_GetComponentToWorld` _dmgarea) (`|MakeArray` "ObjectTypeQuery3" :!type "EObjectTypeQuery Enum") "/Game/EPOC_BP/EPOC_CONTENT/Blueprints/PlayerBlueprints/BP_Player.BP_Player_C" _outactors))
  (for _array_element _outactors_2
    (`GameplayStatics.ApplyDamage` _array_element 0.005 null null "/Game/EPOC_BP/EPOC_CONTENT/Blueprints/DamageTypes/DMG_SlowDamage.DMG_SlowDamage_C")
    (`KismetSystemLibrary.Delay` 0.1)))

(fn `UserConstructionScript`)