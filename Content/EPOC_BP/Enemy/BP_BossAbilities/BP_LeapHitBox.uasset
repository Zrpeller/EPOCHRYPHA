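; Hit box actor for the boss's leap attack that deals area damage to pawns when the boss lands.
; Tick, throttled by Delays, keeps it below its owning boss and sets airborne or landing flags on the boss AI controller.
; On landing it enables the damage area, shows its visual, then clears the attack state and destroys itself.
; The first overlap damages overlapping non-boss pawns and disables collision.
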(event `self.ReceiveBeginPlay`
  (`PrimitiveComponent.SetCollisionEnabled` (`self.dmgArea`) "NoCollision")
  (`SceneComponent.SetVisibility` (`self.dmgTexture`) false false))

(event `self.ReceiveTick`
  (params (DeltaSeconds :type "Float (single-precision)"))
  (bind _returnvalue (`self.GetOwner`))
  (bind (_returnvalue_x _returnvalue_y _returnvalue_z) (`KismetMathLibrary.BreakVector` (`self.K2_GetActorLocation` _returnvalue)))
  (`KismetSystemLibrary.Delay` 0.5)
  (bind _asbp_enemy_boss (cast `/Game/EPOC_BP/Enemy/BossEnemy/BP_Enemy_Boss` _returnvalue))
  (bind _asai_boss (cast `/Game/EPOC_BP/Enemy/BossEnemy/AI_Boss` (`/Game/EPOC_BP/Enemy/BossEnemy/BP_Enemy_Boss.AsBossController` _asbp_enemy_boss)))
  (`self.K2_SetActorLocation` (`KismetMathLibrary.MakeVector` _returnvalue_x _returnvalue_y (- _returnvalue_z 80.0)))
  (if (`NavMovementComponent.IsFalling` (`Character.CharacterMovement` _asbp_enemy_boss))
    (set `/Game/EPOC_BP/Enemy/BossEnemy/AI_Boss.IsLeaping?` false _asai_boss)
    (set `/Game/EPOC_BP/Enemy/BossEnemy/AI_Boss.IsInAir?` true _asai_boss)
    (else
      (set `/Game/EPOC_BP/Enemy/BossEnemy/AI_Boss.IsInAir?` false _asai_boss)
      (set `/Game/EPOC_BP/Enemy/BossEnemy/AI_Boss.IsLanding?` true _asai_boss)
      (`PrimitiveComponent.SetCollisionEnabled` (`self.dmgArea`) "QueryAndPhysics")
      (`KismetSystemLibrary.Delay` 0.2)
      (`SceneComponent.SetVisibility` (`self.dmgTexture`) true false)
      (set `/Game/EPOC_BP/Enemy/BossEnemy/AI_Boss.IsLanding?` false _asai_boss)
      (`KismetSystemLibrary.Delay` 0.5)
      (set `/Game/EPOC_BP/Enemy/BossEnemy/AI_Boss.IsOnGround?` true _asai_boss)
      (`KismetSystemLibrary.Delay` 1.0)
      (set `/Game/EPOC_BP/Enemy/BossEnemy/AI_Boss.IsOnGround?` false _asai_boss)
      (set `/Game/EPOC_BP/Enemy/BossEnemy/AI_Boss.Attacking?` false _asai_boss)
      (`self.K2_DestroyActor`))))

(event `self.dmgArea.OnComponentBeginOverlap`
  (params (OverlappedComponent :type "PrimitiveComponent Object Reference") (OtherActor :type "Actor Object Reference") (OtherComp :type "PrimitiveComponent Object Reference") (OtherBodyIndex :type Integer) (bFromSweep :type Boolean) (SweepResult :type "HitResult Structure (by ref)"))
  (bind _outactors (`GameplayStatics.GetAllActorsOfClass` "/Game/EPOC_BP/Enemy/BossEnemy/BP_Enemy_Boss.BP_Enemy_Boss_C"))
  (bind _outactors_2 (`KismetSystemLibrary.ComponentOverlapActors` (`self.dmgArea`) (`SceneComponent.K2_GetComponentToWorld` (`self.dmgTexture`)) (`|MakeArray` "ObjectTypeQuery3" :!type "EObjectTypeQuery Enum") null _outactors))
  (for _array_element _outactors_2
    (`GameplayStatics.ApplyDamage` _array_element 1.0))
  (`PrimitiveComponent.SetCollisionEnabled` (`self.dmgArea`) "NoCollision"))

(fn `UserConstructionScript`)