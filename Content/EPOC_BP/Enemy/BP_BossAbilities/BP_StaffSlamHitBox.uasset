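; BP_StaffSlamHitBox is a short-lived damage hit box, apparently for a boss staff slam attack.
; Overlapping a BP_ShieldSpecial flags damage as blocked (whatever its ChargeTime) and disables the box's collision.
; Otherwise, an overlapping BP_Player takes a small amount of damage once, unless blocked.
; Delays driven from Tick switch collision off after a brief window, then destroy the actor.
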(event `self.ReceiveTick`
  (params (DeltaSeconds :type "Float (single-precision)"))
  (`KismetSystemLibrary.Delay` 0.2)
  (`PrimitiveComponent.SetCollisionEnabled` (`self.Box`) "NoCollision")
  (`KismetSystemLibrary.Delay` 1.0)
  (`self.K2_DestroyActor`))

(event `self.Box.OnComponentBeginOverlap`
  (params (OverlappedComponent :type "PrimitiveComponent Object Reference") (OtherActor :type "Actor Object Reference") (OtherComp :type "PrimitiveComponent Object Reference") (OtherBodyIndex :type Integer) (bFromSweep :type Boolean) (SweepResult :type "HitResult Structure (by ref)"))
  (bind _asbp_shield_special (cast `/Game/EPOC_BP/EPOC_CONTENT/Blueprints/PlayerBlueprints/KnightPlayer/BP_ShieldSpecial` OtherActor)
    (:`then`
      (if (<= (`/Game/EPOC_BP/EPOC_CONTENT/Blueprints/PlayerBlueprints/KnightPlayer/BP_ShieldSpecial.ChargeTime` _asbp_shield_special) 0.04)
        (set `self.DamageBlocked` true)
        (else
          (set `self.DamageBlocked` true)))
      (`PrimitiveComponent.SetCollisionEnabled` (`self.Box`) "NoCollision"))
    (:`CastFailed`
      (bind _asbp_player (cast `/Game/EPOC_BP/EPOC_CONTENT/Blueprints/PlayerBlueprints/BP_Player` OtherActor))
      (if (not (`self.DamageBlocked`))
        (`/Engine/EditorBlueprintResources/StandardMacros.DoOnce` false
          (:`Completed`
            (`GameplayStatics.ApplyDamage` _asbp_player 0.25)
            (`KismetSystemLibrary.Delay` 0.1)))))))

(fn `UserConstructionScript`)