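; Melee enemy Blueprint that extends a parent enemy, setting its health and attack speed on BeginPlay.
; Tick plays the Brawler death animation whenever health is at or below zero, re-triggering it each frame.
; DamageBox end overlap clears TouchingPlayer for the player unless Dying, while begin overlap does nothing.
; The sword-slash attack loop, which spawns and destroys a temporary hitbox actor, is disconnected and never runs.
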(event `self.ReceiveBeginPlay`
  (`parent.ReceiveBeginPlay`)
  (set `self.AttackSpeed` 0.3)
  (set `self.health` 90.0))

(event `self.ReceiveTick`
  (params (DeltaSeconds :type "Float (single-precision)"))
  (if (<= (`self.health`) 0.0)
    (`SkeletalMeshComponent.PlayAnimation` (`self.Mesh`) "/Game/Character_Rigs/Melee_Enemy/Animations/Brawler_Death_Retargeted.Brawler_Death_Retargeted" false)))

(event `self.DamageBox.OnComponentBeginOverlap`
  (params (OverlappedComponent :type "PrimitiveComponent Object Reference") (OtherActor :type "Actor Object Reference") (OtherComp :type "PrimitiveComponent Object Reference") (OtherBodyIndex :type Integer) (bFromSweep :type Boolean) (SweepResult :type "HitResult Structure (by ref)")))

(event `self.DamageBox.OnComponentEndOverlap`
  (params (OverlappedComponent :type "PrimitiveComponent Object Reference") (OtherActor :type "Actor Object Reference") (OtherComp :type "PrimitiveComponent Object Reference") (OtherBodyIndex :type Integer))
  (if (not (`self.Dying?`))
    (cast `/Game/EPOC_BP/EPOC_CONTENT/Blueprints/PlayerBlueprints/BP_Player` OtherActor)
    (set `self.TouchingPlayer` false)))

(fn `UserConstructionScript`
  (`parent.UserConstructionScript`))