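; Hitbox actor for an archer's arrow that damages BP_Player on overlap and can be blocked by BP_ShieldSpecial.
; Overlapping the shield flags damage as blocked and destroys the arrow; overlapping the player applies a small hit once, then destroys it.
; A short Delay on Tick caps the arrow's lifetime.
; Projectile speed, health and parry logic are left disconnected and never run.
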(event `self.ReceiveActorBeginOverlap`
  (params (OtherActor :type "Actor Object Reference")))

(event `self.ReceiveTick`
  (params (DeltaSeconds :type "Float (single-precision)"))
  ;[1 1 1] For Projectile Speed
  (`KismetSystemLibrary.Delay` 0.7)
  (`self.K2_DestroyActor`))

(event `self.ReceiveBeginPlay`)

(event `self.Cube.OnComponentBeginOverlap`
  (params (OverlappedComponent :type "PrimitiveComponent Object Reference") (OtherActor :type "Actor Object Reference") (OtherComp :type "PrimitiveComponent Object Reference") (OtherBodyIndex :type Integer) (bFromSweep :type Boolean) (SweepResult :type "HitResult Structure (by ref)"))
  (cast `/Game/EPOC_BP/EPOC_CONTENT/Blueprints/PlayerBlueprints/KnightPlayer/BP_ShieldSpecial` OtherActor
    (:`then`
      (`KismetSystemLibrary.PrintString` "Block Damage")
      (set `self.DamageBlocked` true)
      (`self.K2_DestroyActor`))
    (:`CastFailed`
      (bind _asbp_player (cast `/Game/EPOC_BP/EPOC_CONTENT/Blueprints/PlayerBlueprints/BP_Player` OtherActor))
      (if (not (`self.DamageBlocked`))
        (`/Engine/EditorBlueprintResources/StandardMacros.DoOnce` false
          (:`Completed`
            (`GameplayStatics.ApplyDamage` _asbp_player 0.8)
            (`self.K2_DestroyActor`)))))))

(fn `UserConstructionScript`
  ;[1 1 1] Set Speed of Projectile
)