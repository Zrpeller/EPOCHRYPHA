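; BP_Camera is a shared camera rig that keeps a group of active players framed.
; GameStarted stores the player array and enables the Tick update.
; Each tick lerps the Sphere toward the players' average location by MoveSpeed, without delta-time scaling.
; It then sets spring arm length directly to the largest pairwise player distance, clamped between minimum and maximum lengths.
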(event `self.ReceiveTick`
  (params (DeltaSeconds :type "Float (single-precision)"))
  (if (`self.bGamestarted`)
    (`self.CalculateAndUpdateCameraMovement`)
    (`self.UpdateSpringArmLength`)))

(fn `CalculateAndUpdateCameraMovement`
  (set `self.PreviousLocation` (`SceneComponent.K2_GetComponentLocation` (`self.Sphere`)))
  (bind _returnvalue (`GameplayStatics.GetActorArrayAverageLocation` (`self.Active Players`)))
  (`SceneComponent.K2_SetWorldLocation` (`self.Sphere`) (`KismetMathLibrary.VLerp` (`self.PreviousLocation`) _returnvalue (`self.MoveSpeed`)) false false))

(fn `GameStarted`
  (params (ActivePlayers :type "Array of /Game/EPOC_BP/EPOC_CONTENT/Blueprints/BP_Player Object Reference"))
  (set `self.Active Players` ActivePlayers)
  (set `self.bGamestarted` true))

(fn `UpdateSpringArmLength`
  (for (_array_element _array_index) (`self.Active Players`)
    (set `self.CurrentPlayer` _array_element)
    (for _index (range (+ _array_index 1) (`KismetArrayLibrary.Array_Length` (`self.Active Players`)))
      (`KismetArrayLibrary.Array_Add` (`self.Distance`) (`self.GetDistanceTo` (`self.CurrentPlayer`) (`|GetArrayItem` (`self.Active Players`) _index)))))
  (set `SpringArmComponent.TargetArmLength` (`KismetMathLibrary.FClamp` (`.MaxValue` (`KismetMathLibrary.MaxOfFloatArray` (`self.Distance`))) (`self.MinArmLength`) (`self.MaxArmLength`)) (`self.SpringArm`))
  (`KismetArrayLibrary.Array_Clear` (`self.Distance`)))

(fn `UserConstructionScript`)