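; Per-player input receiver for the menu and loss screens, handling player joining and character-select input.
; While not in play on the menu level, Start opens the joining phase, then spawns up to three BP_TestInput actors, possessed via PlayerIndex and ordered by the game instance.
; Start on the loss level reloads the menu; left/right inputs cycle the character menu.
; Older ready-up and character confirmation logic remains disconnected and never runs.
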(event `self.ReceiveBeginPlay`
  (bind _asbp_epochgame_instance (cast `/Game/EPOC_BP/EPOC_CONTENT/Blueprints/BP_EPOCHGameInstance` (`GameplayStatics.GetGameInstance`)))
  (set `self.EPOCH_GameInstance` _asbp_epochgame_instance))

(event `InputAction|Start` :consume false
  (params (Key :type "Key Structure"))
  (bind _playerindex (`self.PlayerIndex`))
  (:`Pressed`
    (if (not (`/Game/EPOC_BP/EPOC_CONTENT/Blueprints/BP_EPOCHGameInstance.InPlay?` (`self.EPOCH_GameInstance`)))
      (bind _returnvalue (`GameplayStatics.GetCurrentLevelName` true))
      (if (`KismetStringLibrary.EqualEqual_StrStr` _returnvalue "BUILD_MenuLevel")
        (bind _outactors (`GameplayStatics.GetAllActorsOfClass` "/Game/EPOC_BP/EPOC_CONTENT/Blueprints/BP_TestInput.BP_TestInput_C"))
        (bind _asbp_epochgame_instance (cast `/Game/EPOC_BP/EPOC_CONTENT/Blueprints/BP_EPOCHGameInstance` (`GameplayStatics.GetGameInstance`)))
        (set `self.EpochInstanceRef` _asbp_epochgame_instance)
        (if (`/Game/EPOC_BP/EPOC_CONTENT/Blueprints/BP_EPOCHGameInstance.PlayersChoosing?` _asbp_epochgame_instance)
          (if (< (`KismetArrayLibrary.Array_Length` _outactors) 3)
            (bind _returnvalue_2 (`|SpawnActorFromClass` "/Game/EPOC_BP/EPOC_CONTENT/Blueprints/BP_TestInput.BP_TestInput_C" (`self.GetTransform` self) "Undefined" "OverrideRootScale" null (`/Game/EPOC_BP/EPOC_CONTENT/Blueprints/BP_EPOCHGameInstance.PlayerOrder` _asbp_epochgame_instance) false _playerindex null))
            (`Controller.Possess` (`GameplayStatics.GetPlayerControllerFromID` _playerindex) _returnvalue_2)
            (`/Game/EPOC_BP/EPOC_CONTENT/Blueprints/BP_EPOCHGameInstance.IncreasePlayerOrder` _asbp_epochgame_instance))
          (else
            (set `/Game/EPOC_BP/EPOC_CONTENT/Blueprints/BP_EPOCHGameInstance.PlayersChoosing?` true _asbp_epochgame_instance)))))))

(event `InputAction|Start` :consume false
  (params (Key :type "Key Structure"))
  (:`Pressed`
    (bind _returnvalue (`GameplayStatics.GetCurrentLevelName` true))
    (if (`KismetStringLibrary.EqualEqual_StrStr` _returnvalue "BUILD_LossLevel")
      (`GameplayStatics.OpenLevel` "BUILD_MenuLevel")
      (set `/Game/EPOC_BP/EPOC_CONTENT/Blueprints/BP_EPOCHGameInstance.InPlay?` true (`self.EPOCH_GameInstance`)))))

(event `Key|Gamepad_FaceButton_Bottom`
  (params (Key :type "Key Structure")))

(event `InputAction|StartGame`
  (params (Key :type "Key Structure")))

(event `InputAction|MenuLeft`
  (params (Key :type "Key Structure"))
  (:`Pressed`
    (`/Engine/EditorBlueprintResources/StandardMacros.IsValid` (`self.CharacterMenuRef`)
      (:`Is Valid`
        (`/Game/EPOC_BP/EPOC_CONTENT/Blueprints/UI/WBP_CharacterSelect.SwitchCharacter` (`self.CharacterMenuRef`) -1)))))

(event `InputAction|MenuRight`
  (params (Key :type "Key Structure"))
  (:`Pressed`
    (`/Engine/EditorBlueprintResources/StandardMacros.IsValid` (`self.CharacterMenuRef`)
      (:`Is Valid`
        (`/Game/EPOC_BP/EPOC_CONTENT/Blueprints/UI/WBP_CharacterSelect.SwitchCharacter` (`self.CharacterMenuRef`) 1)))))

(event `self.ReceiveTick`
  (params (DeltaSeconds :type "Float (single-precision)")))

(fn `UserConstructionScript`)