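; BP_EPOCHGameInstance is a game instance that stores player selection and controller order data.
; GetPlayerInputRecieverValues appends the incoming choice and controller references to two arrays with AddUnique, so repeated entries are ignored.
; IncreasePlayerOrder increments a separate player order counter.
; Unconnected leftover nodes that gather BP_InputReceiver actors and copy their PlayerChoice values never run.
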(fn `getPlayerInputRecieverValues`
  (params (PlayerChoiceRef :type Integer) (ControllerOrderRef :type Integer))
  ;[1 1 1] Store player activity and player selection information
  (`KismetArrayLibrary.Array_AddUnique` (`self.playerChoiceArray`) PlayerChoiceRef)
  (`KismetArrayLibrary.Array_AddUnique` (`self.ControllerOrderArray`) ControllerOrderRef)
  (return))

(fn `IncreasePlayerOrder`
  (set `self.PlayerOrder` (+ (`self.PlayerOrder`) 1))
  (return))