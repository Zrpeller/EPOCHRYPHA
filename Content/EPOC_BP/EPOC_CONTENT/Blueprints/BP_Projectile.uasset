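; BP_Projectile is a projectile actor that moves at a configurable speed and removes itself after a set lifetime.
; The construction script copies ProjectileSpeed into the movement component's InitialSpeed.
; Tick runs a Delay of ProjectileLifeTime, then destroys the actor.
; Overlap events are empty, and the projectile health and hit-destroy logic is disconnected, so collisions have no effect in this graph.
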(event `self.ReceiveActorBeginOverlap`
  (params (OtherActor :type "Actor Object Reference")))

(event `self.projectileCollision.OnComponentBeginOverlap`
  (params (OverlappedComponent :type "PrimitiveComponent Object Reference") (OtherActor :type "Actor Object Reference") (OtherComp :type "PrimitiveComponent Object Reference") (OtherBodyIndex :type Integer) (bFromSweep :type Boolean) (SweepResult :type "HitResult Structure (by ref)")))

(event `self.ReceiveTick`
  (params (DeltaSeconds :type "Float (single-precision)"))
  ;[1 1 1] For Projectile Speed
  (`KismetSystemLibrary.Delay` (`self.ProjectileLifeTime`))
  (`self.K2_DestroyActor`))

(event `self.ReceiveBeginPlay`)

(event `self.projectileCollision.OnComponentEndOverlap`
  (params (OverlappedComponent :type "PrimitiveComponent Object Reference") (OtherActor :type "Actor Object Reference") (OtherComp :type "PrimitiveComponent Object Reference") (OtherBodyIndex :type Integer)))

(fn `UserConstructionScript`
  ;[1 1 1] Set Speed of Projectile
  (bind _output_get (set `ProjectileMovementComponent.InitialSpeed` (`self.ProjectileSpeed`) (`self.ProjectileMovement`))))