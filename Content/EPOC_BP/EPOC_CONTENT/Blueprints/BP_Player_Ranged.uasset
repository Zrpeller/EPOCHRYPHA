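; BP_Player_Ranged is a player Blueprint for a charge-and-release ranged basic attack.
; Pressing BasicAttack, gated by ProjectileDestroyed, attaches a linear telegraph VFX and starts a looping timer that raises a clamped ProjectilePower.
; Releasing removes the telegraph, spawns BP_Projectile with speed, lifetime and damage derived from that power, then resets it.
; An older cooldown workaround remains as unreachable nodes, so live code never changes ProjectileDestroyed.
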(event `InputAction|BasicAttack`
  (params (Key :type "Key Structure"))
  (bind _projectilepower (`self.ProjectilePower`))
  ;[1 1 1] Ranged Player Attacks
  (:`Pressed`
    ;;[1 1 1] Prevent drawing of range if can't fire
    (if (`self.ProjectileDestroyed?`)
      (set `self.IsAttacking?` true)
      (bind _returnvalue (`|SpawnActorFromClass` "/Game/EPOC_BP/VFX_/VFX_Decal/VFX_Actor_LinearSkill.VFX_Actor_LinearSkill_C" (`KismetMathLibrary.MakeTransform` (`SceneComponent.K2_GetComponentLocation` (`self.Mesh`)) (`SceneComponent.K2_GetComponentRotation` (`self.LinearSkillTelegraphPoint`)) (0.1 2.5 0.2)) "Undefined" "OverrideRootScale" null null))
      (bind _output_get (set `self.linearActorRef` _returnvalue))
      (`self.K2_AttachToComponent` _output_get (`self.LinearSkillTelegraphPoint`) "None" "KeepWorld" "KeepWorld" "KeepWorld" true)
      (bind _returnvalue_2 (`KismetSystemLibrary.K2_SetTimer` null "IncreaseProjectilePower" 0.01 true))))
  (:`Released`
    (set `self.IsAttacking?` false)
    (`KismetSystemLibrary.K2_ClearAndInvalidateTimerHandle` _returnvalue_2)
    (`self.K2_DestroyActor` (`self.linearActorRef`))
    (`|SpawnActorFromClass` "/Game/EPOC_BP/EPOC_CONTENT/Blueprints/BP_Projectile.BP_Projectile_C" (`SceneComponent.K2_GetComponentToWorld` (`self.SpawnProjectile`)) "Undefined" "OverrideRootScale" null (+ (* (`self.ProjectilePower`) (`self.ShotMultiplier`)) 1000.0) (/ _projectilepower 30.0) _projectilepower null)
    (`KismetSystemLibrary.PrintString` (`KismetStringLibrary.Conv_DoubleToString` _projectilepower))
    (set `self.ProjectilePower` 20.0)))

(fn `increaseProjectilePower`
  (set `self.ProjectilePower` (`KismetMathLibrary.FClamp` (+ (`self.ProjectilePower`) 1.0) 20.0 75.0)))

(fn `UserConstructionScript`
  (`parent.UserConstructionScript`))