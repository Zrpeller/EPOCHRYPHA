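; BP_LevelSwitchTrigger is a placeable trigger that moves the game to the next level when a player enters it carrying the relic.
; Overlap on the LevelSwitch component casts to BP_Player and checks HasGuffy, then opens the level named in NextLevelName or prints a failure message.
; BeginPlay caches all BP_Player actors in ListOfPlayers, but the overlap logic does not use that list.
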(event `self.ReceiveBeginPlay`
  (bind _outactors (`GameplayStatics.GetAllActorsOfClass` "/Game/EPOC_BP/EPOC_CONTENT/Blueprints/PlayerBlueprints/BP_Player.BP_Player_C"))
  (set `self.listOfPlayers` _outactors))

(event `self.levelSwitch.OnComponentBeginOverlap`
  (params (OverlappedComponent :type "PrimitiveComponent Object Reference") (OtherActor :type "Actor Object Reference") (OtherComp :type "PrimitiveComponent Object Reference") (OtherBodyIndex :type Integer) (bFromSweep :type Boolean) (SweepResult :type "HitResult Structure (by ref)"))
  ;[1 1 1] Switch Level on player entry with relic, jus place in game and set nam variable to the name of the next level
  (bind _asbp_player (cast `/Game/EPOC_BP/EPOC_CONTENT/Blueprints/PlayerBlueprints/BP_Player` OtherActor))
  (if (`/Game/EPOC_BP/EPOC_CONTENT/Blueprints/PlayerBlueprints/BP_Player.hasGuffy` _asbp_player)
    (`GameplayStatics.OpenLevel` (`self.nextLevelName`))
    (else
      (`KismetSystemLibrary.PrintString` "did not win"))))

(fn `UserConstructionScript`)