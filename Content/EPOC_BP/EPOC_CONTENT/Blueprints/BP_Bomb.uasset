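; BP_Bomb is a short-lived bomb actor that damages enemies inside its collision volume and destroys itself after a brief delay following BeginPlay.
; Every Tick, it queries BombCollision for overlapping Enemy pawns, ignoring BombCreator, and applies a small fixed damage to each.
; Damage is not scaled by delta time, so the total dealt over the bomb's lifetime depends on frame rate.
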(event `self.ReceiveBeginPlay`
  (`KismetSystemLibrary.Delay` 2.5)
  (`self.K2_DestroyActor`))

(event `self.ReceiveTick`
  (params (DeltaSeconds :type "Float (single-precision)"))
  (bind _bombcollision (`self.BombCollision`))
  (bind _outactors (`KismetSystemLibrary.ComponentOverlapActors` _bombcollision (`SceneComponent.K2_GetComponentToWorld` _bombcollision) (`|MakeArray` "ObjectTypeQuery3" :!type "EObjectTypeQuery Enum") "/Game/EPOC_BP/Enemy/Enemy.Enemy_C" (`|MakeArray` (`self.BombCreator`))))
  (for _array_element _outactors
    (`GameplayStatics.ApplyDamage` _array_element 0.8)))

(fn `UserConstructionScript`)