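; Game mode that sets up a local multiplayer match from the character choices stored in the game instance.
; On BeginPlay it creates local players with input receivers at tag-indexed PlayerStarts and adds the player HUD.
; It then spawns each chosen ranged, melee or AOE character, possessed via the saved controller order, and registers its HUD status.
; All players view one shared BP_Camera, which receives the player list once spawning finishes.
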(event `self.ReceiveBeginPlay`
  (bind _as_bp_epochgameinstanceref (`self.As BP EPOCHGameInstanceRef`))
  (bind _playerchoicearray (`/Game/EPOC_BP/EPOC_CONTENT/Blueprints/BP_EPOCHGameInstance.playerChoiceArray` _as_bp_epochgameinstanceref))
  (bind _asbp_epochgame_instance (cast `/Game/EPOC_BP/EPOC_CONTENT/Blueprints/BP_EPOCHGameInstance` (`GameplayStatics.GetGameInstance`)))
  (set `self.As BP EPOCHGameInstanceRef` _asbp_epochgame_instance)
  (`self.ActivateCamerasAndPlayers`)
  (bind _returnvalue (`|CreateWidget` "/Game/EPOC_BP/EPOC_CONTENT/Blueprints/UI/WBP_PlayerHUD.WBP_PlayerHUD_C" null true))
  (bind _output_get (set `self.PlayerHUDRef` _returnvalue))
  (`UserWidget.AddToViewport` _output_get 0)
  ;[1 1 1] Get Players and their choices, then spawn them in
  (for (_ _array_index) _playerchoicearray
    (bind _output (`|GetArrayItem` (`self.PlayerInputReceiverArray`) _array_index))
    (bind _playerindex (`/Game/EPOC_BP/EPOC_CONTENT/Blueprints/BP_InputReceiver.PlayerIndex` _output))
    (bind _output_2 (`|GetArrayItem` _playerchoicearray _array_index))
    (`self.SpawnPlayer` self _playerindex _output_2 _output (`|GetArrayItem` (`/Game/EPOC_BP/EPOC_CONTENT/Blueprints/BP_EPOCHGameInstance.ControllerOrderArray` _as_bp_epochgameinstanceref) _array_index))
    (`self.DisplayPlayerStatus` _output_2 _playerindex))
  (`/Game/EPOC_BP/EPOC_CONTENT/Blueprints/BP_Camera.GameStarted` (`self.CameraRef`) (`self.Players`)))

(event `InputAction|StartGame`
  (params (Key :type "Key Structure")))

(fn `ActivateCamerasAndPlayers`
  (bind _outactors (`GameplayStatics.GetAllActorsOfClass` "/Game/EPOC_BP/EPOC_CONTENT/Blueprints/BP_Camera.BP_Camera_C"))
  (set `self.CameraRef` (`|GetArrayItem` _outactors))
  (`self.Set Player Start Points`)
  (`self.SpawnInputReceivers`))

(fn `DisplayCharacterSelect`
  (params (CurrentPlayerIndex :type Integer))
  (returns (Return :type Boolean))
  (bind _characterselect (`/Game/EPOC_BP/EPOC_CONTENT/Blueprints/UI/WBP_Menu.AddCharacterSelect` (`self.MenuWidgetRef`) CurrentPlayerIndex))
  (set `/Game/EPOC_BP/EPOC_CONTENT/Blueprints/BP_InputReceiver.CharacterMenuRef` _characterselect (`|GetArrayItem` (`self.PlayerInputReceiverArray`) (`local.CurrentPlayerIndex`)))
  (return false))

(fn `DisplayPlayerStatus`
  (params (PlayerCharacterChoice :type Integer) (PlayerIndex :type Integer))
  (returns (Return :type Boolean))
  (bind _playerstatus (`/Game/EPOC_BP/EPOC_CONTENT/Blueprints/UI/WBP_PlayerHUD.AddPlayerToHUD` (`self.PlayerHUDRef`) PlayerCharacterChoice PlayerIndex (`|GetArrayItem` (`self.Players`) PlayerIndex)))
  (set `/Game/EPOC_BP/EPOC_CONTENT/Blueprints/BP_InputReceiver.PlayerStatusRef` _playerstatus (`|GetArrayItem` (`self.PlayerInputReceiverArray`) PlayerIndex))
  (return false))

(fn `GetIsIngame`
  (returns (IsInGame :type Boolean))
  (return (`self.bIsInGame`)))

(fn `NameToInt`
  (params (PlayerStart :type "PlayerStart Object Reference"))
  (returns (ReturnValue :type Integer))
  (return (`KismetStringLibrary.Conv_StringToInt` (`KismetStringLibrary.Conv_NameToString` (`PlayerStart.PlayerStartTag` PlayerStart)))))

(fn `RemoveUnusedCamera`
  (bind _outactors (`GameplayStatics.GetAllActorsOfClass` "/Script/Engine.CameraActor"))
  (for _array_element _outactors
    (`self.K2_DestroyActor` _array_element)))

(fn `Set Player Start Points`
  (bind _outactors (`GameplayStatics.GetAllActorsOfClass` "/Script/Engine.PlayerStart"))
  (set `self.PlayerStartArray` _outactors))

(fn `SpawnInputReceivers`
  (locals (Index :type Integer))
  (bind _playerinputreceiverarray (`self.PlayerInputReceiverArray`))
  (bind _returnvalue (`GameplayStatics.GetPlayerController` (`local.Index`)))
  (for (_ _array_index) (`self.PlayerStartArray`)
    (set `local.Index` _array_index)
    (for _array_element (`self.PlayerStartArray`)
      (if (== (`self.NameToInt` _array_element) (`local.Index`))
        (`GameplayStatics.CreatePlayer` -1)
        (bind _returnvalue_2 (`|SpawnActorFromClass` "/Game/EPOC_BP/EPOC_CONTENT/Blueprints/BP_InputReceiver.BP_InputReceiver_C" (`self.GetTransform` (`|GetArrayItem` (`self.PlayerStartArray`) (`local.Index`))) "Undefined" "OverrideRootScale" null (`local.Index`) false null))
        (`KismetArrayLibrary.Array_AddUnique` _playerinputreceiverarray _returnvalue_2)
        (`Controller.Possess` _returnvalue _returnvalue_2)
        (`KismetArrayLibrary.Array_AddUnique` (`self.PlayerControllerArray`) _returnvalue)
        (bind _asbp_epochgame_instance (cast `/Game/EPOC_BP/EPOC_CONTENT/Blueprints/BP_EPOCHGameInstance` (`GameplayStatics.GetGameInstance`)))
        (bind _playerchoicearray (`/Game/EPOC_BP/EPOC_CONTENT/Blueprints/BP_EPOCHGameInstance.playerChoiceArray` _asbp_epochgame_instance))
        (for (_ _array_index_2) _playerchoicearray
          (set `/Game/EPOC_BP/EPOC_CONTENT/Blueprints/BP_InputReceiver.playerChoice` (`|GetArrayItem` _playerchoicearray _array_index_2) (`|GetArrayItem` _playerinputreceiverarray _array_index_2))
          (`self.RemoveUnusedCamera`)
          (`PlayerController.SetViewTargetWithBlend` (`GameplayStatics.GetPlayerController` (`local.Index`)) (`self.CameraRef`) 0.0 "VTBlend_Linear" 0.0 false))))))

(fn `SpawnPlayer`
  (params (CurrentPlayerIndex :type Integer) (CharacterChoice :type Integer) (InputReciever :type "/Game/EPOC_BP/EPOC_CONTENT/Blueprints/BP_InputReceiver Object Reference") (ControllerOrder :type Integer))
  (returns (Return :type Boolean))
  (bind _controllerorder (`local.ControllerOrder`))
  (bind _controllerorder_2 (`local.ControllerOrder`))
  (bind _controllerorder_3 (`local.ControllerOrder`))
  (switch `int` CharacterChoice
    (:`0`
      (bind _returnvalue (`|SpawnActorFromClass` "/Game/EPOC_BP/EPOC_CONTENT/Blueprints/PlayerBlueprints/ArcherPlayer/BP_Player_Ranged.BP_Player_Ranged_C" (`self.GetTransform` (`local.InputReciever`)) "Undefined" "OverrideRootScale" null CharacterChoice 20.0 CurrentPlayerIndex null))
      (`KismetArrayLibrary.Array_Add` (`self.Players`) _returnvalue)
      (`Controller.Possess` (`GameplayStatics.GetPlayerController` _controllerorder_3) _returnvalue)
      (`KismetSystemLibrary.PrintString` "P1")
      (`PlayerController.SetViewTargetWithBlend` (`GameplayStatics.GetPlayerController` _controllerorder_3) (`self.CameraRef`) 0.0 "VTBlend_Linear" 0.0 false)
      (return false))
    (:`1`
      (bind _returnvalue_2 (`|SpawnActorFromClass` "/Game/EPOC_BP/EPOC_CONTENT/Blueprints/PlayerBlueprints/KnightPlayer/BP_Player_Melee_02.BP_Player_Melee_02_C" (`self.GetTransform` (`local.InputReciever`)) "Undefined" "OverrideRootScale" null CharacterChoice 20.0 CurrentPlayerIndex null))
      (`KismetArrayLibrary.Array_Add` (`self.Players`) _returnvalue_2)
      (`Controller.Possess` (`GameplayStatics.GetPlayerController` _controllerorder_2) _returnvalue_2)
      (`KismetSystemLibrary.PrintString` "P2")
      (`PlayerController.SetViewTargetWithBlend` (`GameplayStatics.GetPlayerController` _controllerorder_2) (`self.CameraRef`) 0.0 "VTBlend_Linear" 0.0 false)
      (return false))
    (:`2`
      (bind _returnvalue_3 (`|SpawnActorFromClass` "/Game/EPOC_BP/EPOC_CONTENT/Blueprints/PlayerBlueprints/ShamanPlayer/BP_Player_AOE_02.BP_Player_AOE_02_C" (`self.GetTransform` (`local.InputReciever`)) "Undefined" "OverrideRootScale" null CharacterChoice 20.0 CurrentPlayerIndex null))
      (`KismetArrayLibrary.Array_Add` (`self.Players`) _returnvalue_3)
      (`Controller.Possess` (`GameplayStatics.GetPlayerController` _controllerorder) _returnvalue_3)
      (`KismetSystemLibrary.PrintString` "P3")
      (`PlayerController.SetViewTargetWithBlend` (`GameplayStatics.GetPlayerController` _controllerorder) (`self.CameraRef`) 0.0 "VTBlend_Linear" 0.0 false)
      (return false))))

(fn `StartGame`
  (returns (Return :type Boolean))
  (if (>= (`KismetArrayLibrary.Array_Length` (`self.Players`)) (`self.minimumPlayers`))
    (`|CreateWidget` "/Game/EPOC_BP/EPOC_CONTENT/Blueprints/UI/WBP_PlayerHUD.WBP_PlayerHUD_C" null true)
    (`KismetSystemLibrary.PrintString` "Hud Created")
    (return false)))

(fn `UserConstructionScript`)