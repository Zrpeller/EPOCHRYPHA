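; BP_ArrowRainHitbox is a short-lived damage volume for an arrow rain attack that hurts and slows players inside it.
; Cube overlap with BP_Player starts a Delay-driven loop that repeatedly applies small damage and sets Slowed until the player leaves, without clearing Slowed.
; Overlap with BP_ShieldSpecial blocks damage and destroys the hitbox, which otherwise expires via a Delay on Tick.
; Projectile health, parry and speed logic is disconnected.
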(event `self.ReceiveActorBeginOverlap`
  (params (OtherActor :type "Actor Object Reference")))

(event `self.ReceiveTick`
  (params (DeltaSeconds :type "Float (single-precision)"))
  ;[1 1 1] For Projectile Speed
  (`KismetSystemLibrary.Delay` 0.7)
  (`self.K2_DestroyActor`))

(event `self.ReceiveBeginPlay`)

(event `self.Cube.OnComponentBeginOverlap`
  (params (OverlappedComponent :type "PrimitiveComponent Object Reference") (OtherActor :type "Actor Object Reference") (OtherComp :type "PrimitiveComponent Object Reference") (OtherBodyIndex :type Integer) (bFromSweep :type Boolean) (SweepResult :type "HitResult Structure (by ref)"))
  (cast `/Game/EPOC_BP/EPOC_CONTENT/Blueprints/PlayerBlueprints/KnightPlayer/BP_ShieldSpecial` OtherActor
    (:`then`
      (`KismetSystemLibrary.PrintString` "Block Damage")
      (set `self.DamageBlocked` true)
      (`self.K2_DestroyActor`))
    (:`CastFailed`
      (bind _asbp_player (cast `/Game/EPOC_BP/EPOC_CONTENT/Blueprints/PlayerBlueprints/BP_Player` OtherActor))
      (`KismetSystemLibrary.PrintString` "Hello")
      (set `self.TouchingPlayer?` true)
      (if (`self.DamageBlocked`) :!label _label
        _
        (elif (`self.TouchingPlayer?`)
          (`GameplayStatics.ApplyDamage` _asbp_player 0.1)
          (set `/Game/EPOC_BP/EPOC_CONTENT/Blueprints/PlayerBlueprints/BP_Player.Slowed?` true _asbp_player)
          (`KismetSystemLibrary.Delay` 0.04)
          (goto _label))))))

(event `self.Cube.OnComponentEndOverlap`
  (params (OverlappedComponent :type "PrimitiveComponent Object Reference") (OtherActor :type "Actor Object Reference") (OtherComp :type "PrimitiveComponent Object Reference") (OtherBodyIndex :type Integer))
  (cast `/Game/EPOC_BP/EPOC_CONTENT/Blueprints/PlayerBlueprints/BP_Player` OtherActor)
  (set `self.TouchingPlayer?` false))

(fn `UserConstructionScript`
  ;[1 1 1] Set Speed of Projectile
)