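; BP_EPOCLossMode appears to be the game mode for the loss state, but its live event logic only gathers the level's PlayerStarts on BeginPlay.
; SpawnInputRecievers can create local players and possess input receivers at tag-indexed starts, but its only call is disconnected.
; DisplayCharacterSelect links receivers to select-screen entries, while the other player and game-flow functions are stubs returning false.
; Game-over widget and level-loading nodes are also left unwired.
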(event `self.ReceiveBeginPlay`
  (bind _outactors (`GameplayStatics.GetAllActorsOfClass` "/Script/Engine.PlayerStart"))
  (set `self.PlayerStartArray` _outactors))

(event `self.ReceiveTick`
  (params (DeltaSeconds :type "Float (single-precision)")))

(event `InputAction|Start`
  (params (Key :type "Key Structure")))

(fn `DisplayCharacterSelect`
  (params (CurrentPlayerIndex :type Integer))
  (returns (Return :type Boolean))
  (bind _characterselect (`/Game/EPOC_BP/EPOC_CONTENT/Blueprints/UI/WBP_CharacterSelectMenu.addCharacterSelect` (`self.SelectScreenRef`) CurrentPlayerIndex))
  (set `/Game/EPOC_BP/EPOC_CONTENT/Blueprints/BP_InputReceiver.CharacterMenuRef` _characterselect (`|GetArrayItem` (`self.InputRecieverArray`) CurrentPlayerIndex))
  (return false))

(fn `DisplayPlayerStatus`
  (params (PlayerCharacterChoice :type Integer) (PlayerIndex :type Integer))
  (returns (Return :type Boolean))
  (return false))

(fn `GetIsIngame`
  (returns (IsInGame :type Boolean))
  (return false))

(fn `Name To Int`
  (params (PlayerStart :type "PlayerStart Object Reference"))
  (returns (ReturnValue :type Integer))
  (return (`KismetStringLibrary.Conv_StringToInt` (`KismetStringLibrary.Conv_NameToString` (`PlayerStart.PlayerStartTag` PlayerStart)))))

(fn `SpawnInputRecievers`
  (bind _returnvalue (`GameplayStatics.GetPlayerController` (`self.Index`)))
  (for (_ _array_index) (`self.PlayerStartArray`)
    (set `self.Index` _array_index)
    (for _array_element (`self.PlayerStartArray`)
      (if (== (`self.Name To Int` _array_element) (`self.Index`))
        (`GameplayStatics.CreatePlayer` -1)
        (bind _returnvalue_2 (`|SpawnActorFromClass` "/Game/EPOC_BP/EPOC_CONTENT/Blueprints/BP_InputReceiver.BP_InputReceiver_C" (`self.GetTransform` (`|GetArrayItem` (`self.PlayerStartArray`) (`self.Index`))) "AlwaysSpawn" "OverrideRootScale" null (`self.Index`) false null))
        (`KismetArrayLibrary.Array_AddUnique` (`self.InputRecieverArray`) _returnvalue_2)
        (`Controller.Possess` _returnvalue _returnvalue_2)
        (`KismetArrayLibrary.Array_AddUnique` (`self.PlayerControllerArray`) _returnvalue)))))

(fn `SpawnPlayer`
  (params (CurrentPlayerIndex :type Integer) (CharacterChoice :type Integer) (InputReciever :type "/Game/EPOC_BP/EPOC_CONTENT/Blueprints/BP_InputReceiver Object Reference") (ControllerOrder :type Integer))
  (returns (Return :type Boolean))
  (return false))

(fn `StartGame`
  (returns (Return :type Boolean))
  (return false))

(fn `UserConstructionScript`)