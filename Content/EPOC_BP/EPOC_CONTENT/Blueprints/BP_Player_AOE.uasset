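; BP_Player_AOE is an unfinished player area-of-effect attack meant to scale with charge.
; BasicAttack press calls a timer on ChargeTime, which increments Charge, but the timer has no duration or looping set.
; An unconnected spawn node would create VFX_Actor_CircleSkill at AoeTelegraphPoint with the mesh's rotation, scaled by Charge, so it never runs.
; Nothing handles button release or resets Charge.
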(event `InputAction|BasicAttack`
  (params (Key :type "Key Structure"))
  (:`Pressed`
    (`KismetSystemLibrary.K2_SetTimer` null "ChargeTime")))

(fn `chargeTime`
  (set `self.charge` (+ (`self.charge`) 0.1)))

(fn `UserConstructionScript`
  (`parent.UserConstructionScript`))