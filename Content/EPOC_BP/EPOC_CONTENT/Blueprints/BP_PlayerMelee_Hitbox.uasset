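; Short-lived hitbox actor for the player's melee attack, destroyed by a brief delay started from Tick.
; The first Enemy to overlap its Cube takes damage, has the "Concussed?" blackboard key set on its AI, and is launched along the hitbox's forward vector.
; The hitbox then destroys itself; projectile speed and health logic is left over but never runs.
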(event `self.ReceiveActorBeginOverlap`
  (params (OtherActor :type "Actor Object Reference")))

(event `self.ReceiveTick`
  (params (DeltaSeconds :type "Float (single-precision)"))
  ;[1 1 1] For Projectile Speed
  (`KismetSystemLibrary.Delay` 0.3)
  (`self.K2_DestroyActor`))

(event `self.ReceiveBeginPlay`)

(event `self.Cube.OnComponentBeginOverlap`
  (params (OverlappedComponent :type "PrimitiveComponent Object Reference") (OtherActor :type "Actor Object Reference") (OtherComp :type "PrimitiveComponent Object Reference") (OtherBodyIndex :type Integer) (bFromSweep :type Boolean) (SweepResult :type "HitResult Structure (by ref)"))
  (bind _asenemy (cast `/Game/EPOC_BP/Enemy/Enemy` OtherActor))
  (`/Engine/EditorBlueprintResources/StandardMacros.DoOnce` false
    (:`Completed`
      (`GameplayStatics.ApplyDamage` _asenemy 45.0)
      (`BlackboardComponent.SetValueAsBool` (`AIBlueprintHelperLibrary.GetBlackboard` (`/Game/EPOC_BP/Enemy/Enemy.AsController` _asenemy)) "Concussed?" true)
      (`Character.LaunchCharacter` _asenemy (* (`KismetMathLibrary.GetForwardVector` (`self.K2_GetActorRotation`)) 2400.0) false false)
      (`self.K2_DestroyActor`))))

(fn `UserConstructionScript`
  ;[1 1 1] Set Speed of Projectile
)