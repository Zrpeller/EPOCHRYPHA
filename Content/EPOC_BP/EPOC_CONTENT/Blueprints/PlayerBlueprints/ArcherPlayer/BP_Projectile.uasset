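; Archer player projectile that damages enemies, piercing through them only when its damage is high enough to count as fully charged.
; The construction script feeds its speed variable into the movement component, and a Delay on Tick destroys it after its lifetime.
; On overlap, weaker shots are destroyed after damaging an enemy.
; Hitting a BP_RangedWall replaces it with a BP_SpecialProjectile with boosted speed, lifetime and damage.
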(event `self.ReceiveActorBeginOverlap`
  (params (OtherActor :type "Actor Object Reference")))

(event `self.ReceiveTick`
  (params (DeltaSeconds :type "Float (single-precision)"))
  ;[1 1 1] For Projectile Speed
  (`KismetSystemLibrary.Delay` (`self.ProjectileLifeTime`))
  (`self.K2_DestroyActor`))

(event `self.ReceiveBeginPlay`)

(event `self.projectileCollision.OnComponentEndOverlap`
  (params (OverlappedComponent :type "PrimitiveComponent Object Reference") (OtherActor :type "Actor Object Reference") (OtherComp :type "PrimitiveComponent Object Reference") (OtherBodyIndex :type Integer)))

(event `self.projectileCollision.OnComponentBeginOverlap`
  (params (OverlappedComponent :type "PrimitiveComponent Object Reference") (OtherActor :type "Actor Object Reference") (OtherComp :type "PrimitiveComponent Object Reference") (OtherBodyIndex :type Integer) (bFromSweep :type Boolean) (SweepResult :type "HitResult Structure (by ref)"))
  (bind _projectiledamage (`self.ProjectileDamage`))
  (bind _sphere (`self.Sphere`))
  ;[1 1 1] Destroy the projectile if not fully charged. This removes the piercing from spammed projectiles
  (cast `/Game/EPOC_BP/Enemy/BP_Enemy` OtherActor
    (:`then`
      (if (>= _projectiledamage 75.0)
        (`GameplayStatics.ApplyDamage` OtherActor _projectiledamage)
        (else
          (set `ProjectileMovementComponent.MaxSpeed` 0.0 (`self.ProjectileMovement`))
          (`GameplayStatics.ApplyDamage` OtherActor _projectiledamage)
          (`self.K2_DestroyActor`))))
    (:`CastFailed`
      (cast `/Game/EPOC_BP/EPOC_CONTENT/Blueprints/PlayerBlueprints/ArcherPlayer/BP_RangedWall` OtherActor)
      (`|SpawnActorFromClass` "/Game/EPOC_BP/EPOC_CONTENT/Blueprints/PlayerBlueprints/ArcherPlayer/BP_SpecialProjectile.BP_SpecialProjectile_C" (`KismetMathLibrary.MakeTransform` (`SceneComponent.K2_GetComponentLocation` _sphere) (`SceneComponent.K2_GetComponentRotation` _sphere)) "Undefined" "OverrideRootScale" null (* (`self.ProjectileSpeed`) 10.0) (* (`self.ProjectileLifeTime`) 2.0) (* (`self.ProjectileDamage`) 1.25) null)
      (`self.K2_DestroyActor`))))

(fn `UserConstructionScript`
  ;[1 1 1] Set Speed of Projectile
  (bind _output_get (set `ProjectileMovementComponent.InitialSpeed` (`self.ProjectileSpeed`) (`self.ProjectileMovement`)))
  (if (>= _output_get 75.0)
    _))