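; Special archer projectile that damages enemies it overlaps without being destroyed and spawns explosions as it bounces.
; The construction script applies ProjectileSpeed to the movement component and grants more bounces at higher speed tiers.
; Bounces, hits and Cover overlaps spawn BP_ProjectileExplosion, with a second, stronger one on Cover hits.
; It destroys itself when bounces run out or after a lifetime Delay driven from Tick.
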(event `self.ReceiveActorBeginOverlap`
  (params (OtherActor :type "Actor Object Reference")))

(event `self.ReceiveTick`
  (params (DeltaSeconds :type "Float (single-precision)"))
  ;[1 1 1] For Projectile Speed
  (`KismetSystemLibrary.Delay` (`self.ProjectileLifeTime`))
  (`self.K2_DestroyActor`))

(event `self.ReceiveBeginPlay`)

(event `self.projectileCollision.OnComponentEndOverlap`
  (params (OverlappedComponent :type "PrimitiveComponent Object Reference") (OtherActor :type "Actor Object Reference") (OtherComp :type "PrimitiveComponent Object Reference") (OtherBodyIndex :type Integer)))

(event `self.projectileCollision.OnComponentBeginOverlap`
  (params (OverlappedComponent :type "PrimitiveComponent Object Reference") (OtherActor :type "Actor Object Reference") (OtherComp :type "PrimitiveComponent Object Reference") (OtherBodyIndex :type Integer) (bFromSweep :type Boolean) (SweepResult :type "HitResult Structure (by ref)"))
  ;[1 1 1] Destroy the projectile if not fully charged. This removes the piercing from spammed projectiles
  (if (`self.ActorHasTag` OtherActor "Cover")
    (`|SpawnActorFromClass` "/Game/EPOC_BP/EPOC_CONTENT/Blueprints/PlayerBlueprints/ArcherPlayer/BP_ProjectileExplosion.BP_ProjectileExplosion_C" (`KismetMathLibrary.MakeTransform` (`SceneComponent.K2_GetComponentLocation` (`self.projectileCollision`)) (struct) (6.0 6.0 6.0)) "Undefined" "OverrideRootScale" null 0.0 1.0 50.0 null)
    (elif (`self.ActorHasTag` OtherActor "Enemy")
      (`GameplayStatics.ApplyDamage` OtherActor (`self.ProjectileDamage`)))))

(event `self.ProjectileMovement.OnProjectileBounce`
  (params (ImpactResult :type "HitResult Structure (by ref)") (ImpactVelocity :type "Vector Structure (by ref)"))
  (bind _bounces (`self.Bounces`))
  ;[1 1 1] Use this to limit the amount of bounces that can occur
  (set `self.Bounces` (- _bounces 1))
  (`|SpawnActorFromClass` "/Game/EPOC_BP/EPOC_CONTENT/Blueprints/PlayerBlueprints/ArcherPlayer/BP_ProjectileExplosion.BP_ProjectileExplosion_C" (`KismetMathLibrary.MakeTransform` (`SceneComponent.K2_GetComponentLocation` (`self.projectileCollision`)) (struct) (6.0 6.0 6.0)) "Undefined" "OverrideRootScale" null 0.0 1.0 50.0 null)
  (if (<= _bounces 0)
    (`self.K2_DestroyActor`)))

(event `self.projectileCollision.OnComponentHit`
  (params (HitComponent :type "PrimitiveComponent Object Reference") (OtherActor :type "Actor Object Reference") (OtherComp :type "PrimitiveComponent Object Reference") (NormalImpulse :type "Vector Structure") (Hit :type "HitResult Structure (by ref)"))
  (`|SpawnActorFromClass` "/Game/EPOC_BP/EPOC_CONTENT/Blueprints/PlayerBlueprints/ArcherPlayer/BP_ProjectileExplosion.BP_ProjectileExplosion_C" (`KismetMathLibrary.MakeTransform` (`SceneComponent.K2_GetComponentLocation` (`self.projectileCollision`)) (struct) (6.0 6.0 6.0)) "Undefined" "OverrideRootScale" null 0.0 1.0 50.0 null)
  (if (`self.ActorHasTag` OtherActor "Cover")
    (`|SpawnActorFromClass` "/Game/EPOC_BP/EPOC_CONTENT/Blueprints/PlayerBlueprints/ArcherPlayer/BP_ProjectileExplosion.BP_ProjectileExplosion_C" (`KismetMathLibrary.MakeTransform` (`SceneComponent.K2_GetComponentLocation` (`self.projectileCollision`)) (struct) (6.0 6.0 6.0)) "Undefined" "OverrideRootScale" null 0.0 1.0 75.0 null)))

(fn `UserConstructionScript`
  (bind _projectilespeed (`self.ProjectileSpeed`))
  ;[1 1 1] Set Speed of Projectile
  (set `ProjectileMovementComponent.InitialSpeed` _projectilespeed (`self.ProjectileMovement`))
  (if (== _projectilespeed 25000.0)
    (set `self.Bounces` 6)
    (elif (>= _projectilespeed 20000.0)
      (set `self.Bounces` 4)
      (else
        (set `self.Bounces` 2)))))