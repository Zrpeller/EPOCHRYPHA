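; BP_RangedWall is a wall actor for the Archer player that attaches a laser beam wall sound to its Cube component on BeginPlay.
; Its construction script adds itself to AnchorActors and, when that array holds two entries, loops over them with an empty body.
; The anchor logic is unfinished, with an unconnected distance check and no active overlap or tick behavior.
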(event `self.ReceiveBeginPlay`
  (`GameplayStatics.SpawnSoundAttached` "/Game/Audio/sfx/ArcherSFX/Laser_beam_wall_.Laser_beam_wall_" (`self.Cube`) "None" (0.0 0.0 0.0) (struct) "KeepRelativeOffset" false 1.0 1.0 0.0 null null))

(fn `UserConstructionScript`
  (bind _anchoractors (`self.AnchorActors`))
  (`KismetArrayLibrary.Array_Add` _anchoractors self)
  (if (== (`KismetArrayLibrary.Array_Length` _anchoractors) 2)
    (for _array_element _anchoractors
      _)))