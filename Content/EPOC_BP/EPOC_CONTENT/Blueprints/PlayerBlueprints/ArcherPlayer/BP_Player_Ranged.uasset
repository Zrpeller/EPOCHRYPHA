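; Ranged (archer) player character with a charged projectile attack and a two-pylon wall special.
; Holding BasicAttack shows an aim telegraph while a timer builds power, which sets projectile speed, lifetime and damage on release.
; SpecialAttack drops anchors, replacing them alternately, and stretches a wall between them from their midpoint.
; Special energy drains while both anchors exist, removing them and the wall when empty; key 1 spawns a boss.
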(event `self.ReceiveBeginPlay`
  (`KismetSystemLibrary.K2_SetTimer` null "SpecialEnergyTimer" 0.01 true))

(event `self.ReceiveTick`
  (params (DeltaSeconds :type "Float (single-precision)"))
  (`parent.ReceiveTick` DeltaSeconds)
  (if (<= (`self.SpecialEnergy`) 0.0)
    (`KismetArrayLibrary.Array_Clear` (`self.SpecialAnchors`))
    (`self.K2_DestroyActor` (`self.Pylon1`))
    (`self.K2_DestroyActor` (`self.Pylon2`))
    (`self.K2_DestroyActor` (`self.RangedWall`))
    (set `self.Pylon1` null)
    (set `self.Pylon2` null)
    (set `self.Pylon1LastPlaced?` false)))

(event `InputAction|BasicAttack`
  (params (Key :type "Key Structure"))
  (bind _projectilepower (`self.ProjectilePower`))
  (bind (_returnvalue_location _returnvalue_rotation) (`KismetMathLibrary.BreakTransform` (`SceneComponent.K2_GetComponentToWorld` (`self.SpawnProjectile`))))
  ;[1 1 1] Ranged Player Attacks
  (:`Pressed`
    ;;[1 1 1] Prevent drawing of range if can't fire
    (if (`self.ProjectileDestroyed?`)
      (set `self.IsAttacking?` true)
      (bind _returnvalue (`|SpawnActorFromClass` "/Game/EPOC_BP/VFX_/VFX_Decal/VFX_Actor_LinearSkill.VFX_Actor_LinearSkill_C" (`KismetMathLibrary.MakeTransform` (`SceneComponent.K2_GetComponentLocation` (`self.Mesh`)) (`SceneComponent.K2_GetComponentRotation` (`self.LinearSkillTelegraphPoint`)) (0.1 2.5 0.2)) "Undefined" "OverrideRootScale" null null))
      (bind _output_get (set `self.linearActorRef` _returnvalue))
      (`self.K2_AttachToComponent` _output_get (`self.LinearSkillTelegraphPoint`) "None" "KeepWorld" "KeepWorld" "KeepWorld" true)
      (bind _returnvalue_2 (`KismetSystemLibrary.K2_SetTimer` null "IncreaseProjectilePower" 0.01 true))))
  (:`Released`
    (set `self.IsAttacking?` false)
    (`KismetSystemLibrary.K2_ClearAndInvalidateTimerHandle` _returnvalue_2)
    (`self.K2_DestroyActor` (`self.linearActorRef`))
    (`|SpawnActorFromClass` "/Game/EPOC_BP/EPOC_CONTENT/Blueprints/PlayerBlueprints/ArcherPlayer/BP_Projectile.BP_Projectile_C" (`KismetMathLibrary.MakeTransform` _returnvalue_location _returnvalue_rotation (2.0 0.5 0.5)) "Undefined" "OverrideRootScale" null (+ (* (`self.ProjectilePower`) (`self.ShotMultiplier`)) 1000.0) (/ _projectilepower 30.0) _projectilepower null)
    (`KismetSystemLibrary.PrintString` (`KismetStringLibrary.Conv_DoubleToString` _projectilepower))
    (set `self.ProjectilePower` 20.0)))

(event `InputAction|SpecialAttack`
  (params (Key :type "Key Structure"))
  (bind _specialanchors (`self.SpecialAnchors`))
  (bind _mesh (`self.Mesh`))
  (bind _returnvalue (`SceneComponent.K2_GetComponentLocation` _mesh))
  (bind _returnvalue_2 (`SceneComponent.K2_GetComponentRotation` _mesh))
  (bind _returnvalue_3 (`SceneComponent.K2_GetComponentLocation` (`Actor.RootComponent` (`self.Pylon1`))))
  (bind _returnvalue_4 (`SceneComponent.K2_GetComponentLocation` (`Actor.RootComponent` (`self.Pylon2`))))
  ;[1 1 1] Special Attack
  (:`Pressed`
    (if (< (`KismetArrayLibrary.Array_Length` _specialanchors) 2)
      (bind _returnvalue_5 (`|SpawnActorFromClass` "/Game/EPOC_BP/EPOC_CONTENT/Blueprints/PlayerBlueprints/ArcherPlayer/BP_RangedAnchor.BP_RangedAnchor_C" (`KismetMathLibrary.MakeTransform` _returnvalue _returnvalue_2) "Undefined" "OverrideRootScale" null null))
      (if (== (`self.Pylon1`) null)
        (set `self.Pylon1` _returnvalue_5)
        (else
          (bind _output_get (set `self.Pylon2` _returnvalue_5))))
      (`KismetArrayLibrary.Array_Add` _specialanchors _returnvalue_5)
      (if (not (== _output_get null))
        (`KismetSystemLibrary.PrintString` "Hello")
        (if (not (== (`self.RangedWall`) null)) :!label _label
          (`self.K2_DestroyActor` (`self.RangedWall`)))
        (bind _returnvalue_6 (`|SpawnActorFromClass` "/Game/EPOC_BP/EPOC_CONTENT/Blueprints/PlayerBlueprints/ArcherPlayer/BP_RangedWall.BP_RangedWall_C" (`KismetMathLibrary.MakeTransform` (/ (+ _returnvalue_3 _returnvalue_4) (2.0 2.0 2.0)) (`KismetMathLibrary.FindLookAtRotation` _returnvalue_4 _returnvalue_3) (`KismetMathLibrary.MakeVector` (/ (`KismetMathLibrary.Vector_Distance` (`SceneComponent.K2_GetComponentLocation` (`Actor.RootComponent` (`self.Pylon1`))) (`SceneComponent.K2_GetComponentLocation` (`Actor.RootComponent` (`self.Pylon2`)))) 100.0) 1.0 1.0)) "Undefined" "OverrideRootScale" null null))
        (set `self.RangedWall` _returnvalue_6))
      (elif (`self.Pylon1LastPlaced?`)
        (`self.K2_DestroyActor` (`self.Pylon2`))
        (bind _returnvalue_7 (`|SpawnActorFromClass` "/Game/EPOC_BP/EPOC_CONTENT/Blueprints/PlayerBlueprints/ArcherPlayer/BP_RangedAnchor.BP_RangedAnchor_C" (`KismetMathLibrary.MakeTransform` _returnvalue _returnvalue_2) "Undefined" "OverrideRootScale" null null))
        (set `self.Pylon2` _returnvalue_7)
        (set `self.Pylon1LastPlaced?` false)
        (goto _label)
        (else
          (`self.K2_DestroyActor` (`self.Pylon1`))
          (bind _returnvalue_8 (`|SpawnActorFromClass` "/Game/EPOC_BP/EPOC_CONTENT/Blueprints/PlayerBlueprints/ArcherPlayer/BP_RangedAnchor.BP_RangedAnchor_C" (`KismetMathLibrary.MakeTransform` _returnvalue _returnvalue_2) "Undefined" "OverrideRootScale" null null))
          (set `self.Pylon1` _returnvalue_8)
          (set `self.Pylon1LastPlaced?` true)
          (goto _label)))))
  (:`Released`
    (if true
      _)))

(event `InputAction|SpecialAttack`
  (params (Key :type "Key Structure")))

(event `Key|One`
  (params (Key :type "Key Structure"))
  (:`Pressed`
    (`|SpawnActorFromClass` "/Game/EPOC_BP/Enemy/BossEnemy/BP_Enemy_Boss.BP_Enemy_Boss_C" (`SceneComponent.GetRelativeTransform` (`self.CapsuleComponent`)) "Undefined" "OverrideRootScale" null null)))

(fn `increaseProjectilePower`
  (set `self.ProjectilePower` (`KismetMathLibrary.FClamp` (+ (`self.ProjectilePower`) 1.0) 20.0 75.0)))

(fn `SpecialEnergyTimer`
  (bind _specialenergy (`self.SpecialEnergy`))
  (if (< (`KismetArrayLibrary.Array_Length` (`self.SpecialAnchors`)) 2)
    (bind _output_get (set `self.SpecialEnergy` (`KismetMathLibrary.FClamp` (+ _specialenergy 0.01) 0.0 15.0)))
    (else
      ;[1 1 1] Increase the max to increase the speed and power of projectile
      (bind _output_get_2 (set `self.SpecialEnergy` (`KismetMathLibrary.FClamp` (- _specialenergy 0.01) 0.0 15.0))))))

(fn `UserConstructionScript`
  (`parent.UserConstructionScript`))