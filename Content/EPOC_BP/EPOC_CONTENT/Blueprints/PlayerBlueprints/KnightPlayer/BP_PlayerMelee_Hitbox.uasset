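; Short-lived melee hitbox actor, filed under the Knight player, that damages enemies overlapping its box and destroys itself after a brief delay started from Tick.
; A BP_Enemy with an AI_Enemy_Controller takes damage, is concussed through that controller, is launched along the hitbox's forward vector, and consumes the hitbox.
; Other actors tagged Enemy only take damage.
; Projectile speed and health logic is left over and unused.
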(event `self.ReceiveActorBeginOverlap`
  (params (OtherActor :type "Actor Object Reference")))

(event `self.ReceiveTick`
  (params (DeltaSeconds :type "Float (single-precision)"))
  ;[1 1 1] For Projectile Speed
  (`KismetSystemLibrary.Delay` 0.3)
  (`self.K2_DestroyActor`))

(event `self.ReceiveBeginPlay`)

(event `self.Box.OnComponentBeginOverlap`
  (params (OverlappedComponent :type "PrimitiveComponent Object Reference") (OtherActor :type "Actor Object Reference") (OtherComp :type "PrimitiveComponent Object Reference") (OtherBodyIndex :type Integer) (bFromSweep :type Boolean) (SweepResult :type "HitResult Structure (by ref)"))
  (bind _asbp_enemy (cast `/Game/EPOC_BP/Enemy/BP_Enemy` OtherActor)
    (:`then`
      (bind _asai_enemy_controller (cast `/Game/EPOC_BP/Enemy/AI_Enemy_Controller` (`/Game/EPOC_BP/Enemy/BP_Enemy.AsController` _asbp_enemy)))
      (`GameplayStatics.ApplyDamage` _asbp_enemy 45.0)
      (`/Game/EPOC_BP/Enemy/AI_Enemy_Controller.ConcussEnemy` _asai_enemy_controller 0.9 true)
      (`Character.LaunchCharacter` _asbp_enemy (* (`KismetMathLibrary.GetForwardVector` (`self.K2_GetActorRotation`)) 2000.0) false false)
      (`self.K2_DestroyActor`))
    (:`CastFailed`
      (if (`self.ActorHasTag` OtherActor "Enemy")
        (`GameplayStatics.ApplyDamage` OtherActor 45.0)))))

(fn `UserConstructionScript`
  ;[1 1 1] Set Speed of Projectile
)