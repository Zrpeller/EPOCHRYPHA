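; Melee knight player character with a basic attack and a charged shield-bash special that block each other while active.
; Holding basic attack shows an attached sector telegraph; releasing swaps it for a spawned hitbox actor.
; Holding special spawns a shield while a looping timer builds charge; releasing launches the knight, scaling damage and knockback on overlapped enemies and setting their blackboard concussed flag.
; A timer-driven cooldown follows the bash; the sword line-trace timer is disconnected.
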(event `self.ReceiveBeginPlay`
  (`PrimitiveComponent.SetCollisionEnabled` (`self.BashHitBox`) "NoCollision")
  (set `self.MovementSpeed` 1400.0))

(event `self.ReceiveTick`
  (params (DeltaSeconds :type "Float (single-precision)"))
  (`parent.ReceiveTick` DeltaSeconds))

(event `InputAction|BasicAttack`
  (params (Key :type "Key Structure"))
  (bind _mesh (`self.Mesh`))
  (bind _meleehitbox (`self.MeleeHitBox`))
  (:`Pressed`
    (if (not (`self.IsSpecialAttacking?`))
      (set `self.IsAttacking?` true)
      (bind _returnvalue (`|SpawnActorFromClass` "/Game/EPOC_BP/VFX_/VFX_Decal/VFX_Actor_SectorSkill.VFX_Actor_SectorSkill_C" (`KismetMathLibrary.MakeTransform` (`SceneComponent.K2_GetComponentLocation` _mesh) (`SceneComponent.K2_GetComponentRotation` _mesh)) "Undefined" "OverrideRootScale" null null))
      (bind _output_get (set `self.sectorTelegraphRef` _returnvalue))
      (`self.K2_AttachToComponent` _output_get (`self.Mesh`) "None" "KeepWorld" "KeepWorld" "KeepWorld" true)))
  (:`Released`
    (if (`self.IsAttacking?`)
      (set `self.IsAttacking?` false)
      (`self.K2_DestroyActor` (`self.sectorTelegraphRef`))
      (bind _returnvalue_2 (`|SpawnActorFromClass` "/Game/EPOC_BP/EPOC_CONTENT/Blueprints/BP_PlayerMelee_Hitbox.BP_PlayerMelee_Hitbox_C" (`KismetMathLibrary.MakeTransform` (`SceneComponent.K2_GetComponentLocation` _meleehitbox) (`SceneComponent.K2_GetComponentRotation` _meleehitbox) (2.0 2.0 0.05)) "Undefined" "OverrideRootScale" null 0.0 0.0 0.0 null))
      (`self.K2_AttachToComponent` _returnvalue_2 null "None" "KeepWorld" "KeepWorld" "KeepWorld" true)
      (`KismetSystemLibrary.Delay` 0.46))))

(event `triggerSword`)

(event `swordLineTrace`
  (bind _sword (`self.sword`))
  (bind _outactors (`GameplayStatics.GetAllActorsOfClass` "/Game/EPOC_BP/EPOC_CONTENT/Blueprints/PlayerBlueprints/BP_Player.BP_Player_C"))
  (bind _outhit (`KismetSystemLibrary.LineTraceSingle` (`SceneComponent.GetSocketLocation` _sword "start") (`SceneComponent.GetSocketLocation` _sword "end") "TraceTypeQuery2" false _outactors "ForDuration" true (struct :`R` 1.0) (struct :`G` 1.0) 0.01))
  (`GameplayStatics.ApplyDamage` (`.HitActor` (`GameplayStatics.BreakHitResult` _outhit)) 30.0))

(event `stopTriggerSword`
  (`KismetSystemLibrary.K2_ClearAndInvalidateTimerHandle` (`self.triggerSwordEvent`)))

(event `InputAction|SpecialAttack`
  (params (Key :type "Key Structure"))
  (bind _bashcharge (`self.BashCharge`))
  (bind (_returnvalue_location _returnvalue_rotation) (`KismetMathLibrary.BreakTransform` (`SceneComponent.K2_GetComponentToWorld` (`self.ShieldHitbox`))))
  (:`Pressed`
    (if (`self.IsAttacking?`)
      _
      (elif (<= (`self.SpecialCooldownTimer`) 0.0)
        (if (not (`self.SpecialActive?`))
          (set `self.IsSpecialAttacking?` true)
          (set `self.BashCharge` 0.0)
          (bind _returnvalue (`|SpawnActorFromClass` "/Game/EPOC_BP/EPOC_CONTENT/Blueprints/PlayerBlueprints/KnightPlayer/BP_ShieldSpecial.BP_ShieldSpecial_C" (`KismetMathLibrary.MakeTransform` _returnvalue_location _returnvalue_rotation (3.0 1.0 3.0)) "Undefined" "OverrideRootScale" null null))
          (bind _output_get (set `self.ShieldProjectile` _returnvalue))
          (`self.K2_AttachToComponent` _output_get (`self.ShieldHitbox`) "None" "KeepWorld" "KeepWorld" "KeepWorld" true)
          (bind _returnvalue_2 (`KismetSystemLibrary.K2_SetTimer` null "ChargeBash" 0.01 true))))))
  (:`Released`
    (if (`self.IsSpecialAttacking?`)
      (if (not (`self.SpecialActive?`))
        (set `self.SpecialActive?` true)
        (`PrimitiveComponent.SetCollisionEnabled` (`self.BashHitBox`) "QueryAndPhysics")
        (`self.LaunchCharacter` (* (`KismetMathLibrary.GetForwardVector` (`self.K2_GetActorRotation`)) (* _bashcharge 36000.0)))
        (set `self.BashDamage` _bashcharge)
        (`KismetSystemLibrary.K2_ClearAndInvalidateTimerHandle` _returnvalue_2)
        (if (<= (`KismetMathLibrary.VSize` (`MovementComponent.Velocity` (`self.CharacterMovement`))) 0.0)
          (`KismetSystemLibrary.Delay` 0.2)
          (`self.K2_DestroyActor` (`self.ShieldProjectile`))
          (`PrimitiveComponent.SetCollisionEnabled` (`self.BashHitBox`) "NoCollision")
          (set `self.SpecialCooldownTimer` 0.4)
          (`KismetSystemLibrary.K2_SetTimer` null "SpecialCooldown" 0.01 true)
          (set `self.SpecialActive?` false)
          (set `self.IsSpecialAttacking?` false))))))

(event `self.BashHitBox.OnComponentBeginOverlap`
  (params (OverlappedComponent :type "PrimitiveComponent Object Reference") (OtherActor :type "Actor Object Reference") (OtherComp :type "PrimitiveComponent Object Reference") (OtherBodyIndex :type Integer) (bFromSweep :type Boolean) (SweepResult :type "HitResult Structure (by ref)"))
  (bind _asenemy (cast `/Game/EPOC_BP/Enemy/Enemy` OtherActor))
  (if (`self.SpecialActive?`)
    (`GameplayStatics.ApplyDamage` _asenemy (+ (* (`self.BashDamage`) 120.0) 30.0))
    (`KismetSystemLibrary.PrintString` "Hello")
    (`BlackboardComponent.SetValueAsBool` (`AIBlueprintHelperLibrary.GetBlackboard` (`/Game/EPOC_BP/Enemy/Enemy.AsController` _asenemy)) "Concussed?" true)
    (`self.LaunchCharacter` _asenemy (* (`KismetMathLibrary.GetForwardVector` (`self.K2_GetActorRotation`)) (* (`self.BashDamage`) 24000.0)) false false)))

(fn `ChargeBash`
  (set `self.BashCharge` (`KismetMathLibrary.FClamp` (+ (`self.BashCharge`) 0.01) 0.0 0.27)))

(fn `SpecialCooldown`
  (set `self.SpecialCooldownTimer` (`KismetMathLibrary.FClamp` (- (`self.SpecialCooldownTimer`) 0.01) 0.0 0.4)))

(fn `UserConstructionScript`
  (`parent.UserConstructionScript`))