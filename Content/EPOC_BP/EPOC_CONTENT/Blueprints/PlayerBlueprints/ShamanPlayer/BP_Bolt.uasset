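; BP_Bolt is a short-lived blast actor for the Shaman player's special attack, dealing massive damage to enemies in its radius.
; On BeginPlay it spawns the blast VFX on BlastRadius and flags every BP_Bomb in the level, tracked as clouds, as empowered.
; BlastRadius overlaps damage Enemy pawns inside while ignoring players.
; A Delay on Tick destroys the actor a fraction of a second after spawning.
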(event `self.ReceiveBeginPlay`
  (bind _activeclouds (`self.activeClouds`))
  (bind (_returnvalue_roll _returnvalue_pitch _returnvalue_yaw) (`KismetMathLibrary.BreakRotator` (`KismetMathLibrary.MakeRotFromX` (`SceneComponent.GetForwardVector` (`self.startPoint`)))))
  (bind _outactors (`GameplayStatics.GetAllActorsOfClass` "/Game/EPOC_BP/EPOC_CONTENT/Blueprints/PlayerBlueprints/BP_Player.BP_Player_C"))
  (set `self.activePlayers` _outactors)
  (bind _outactors_2 (`GameplayStatics.GetAllActorsOfClass` "/Game/EPOC_BP/EPOC_CONTENT/Blueprints/PlayerBlueprints/ShamanPlayer/BP_Bomb.BP_Bomb_C"))
  (set `self.activeClouds` _outactors_2)
  (bind _returnvalue (`NiagaraFunctionLibrary.SpawnSystemAttached` "/Game/VFX_/VFX_Shaman/VFX_Shaman_Dash/VFX__Shaman_BlastSpecial.VFX__Shaman_BlastSpecial" (`self.blastRadius`) "None" (`SceneComponent.K2_GetComponentLocation` (`Actor.RootComponent` (`self.caster`))) (`KismetMathLibrary.MakeRotator` 0.0 0.0 _returnvalue_yaw) "SnapToTargetIncludingScale"))
  (set `self.boltVFX` _returnvalue)
  (for (_ _array_index) _activeclouds
    (set `/Game/EPOC_BP/EPOC_CONTENT/Blueprints/PlayerBlueprints/ShamanPlayer/BP_Bomb.isEmpowered` true (`|GetArrayItem` _activeclouds _array_index))))

(event `self.ReceiveTick`
  (params (DeltaSeconds :type "Float (single-precision)"))
  (`KismetSystemLibrary.Delay` 0.1)
  (`self.K2_DestroyActor` self))

(event `self.blastRadius.OnComponentBeginOverlap`
  (params (OverlappedComponent :type "PrimitiveComponent Object Reference") (OtherActor :type "Actor Object Reference") (OtherComp :type "PrimitiveComponent Object Reference") (OtherBodyIndex :type Integer) (bFromSweep :type Boolean) (SweepResult :type "HitResult Structure (by ref)"))
  (bind _outactors (`KismetSystemLibrary.ComponentOverlapActors` (`self.blastRadius`) (`SceneComponent.K2_GetComponentToWorld` (`self.blastRadius`)) (`|MakeArray` "ObjectTypeQuery3" :!type "EObjectTypeQuery Enum") "/Game/EPOC_BP/Enemy/Enemy.Enemy_C" (`self.activePlayers`)))
  (for _array_element _outactors
    (`GameplayStatics.ApplyDamage` _array_element 10000.0)))

(fn `UserConstructionScript`)