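; Shaman player character with a targeted bomb, a lightning bolt special and a teleport replacing the parent dash.
; Holding basic attack charges while movement input steers a range-clamped telegraph, where release spawns BP_Bomb if charged enough.
; Special spawns BP_Bolt on a timer-driven cooldown, while jump teleports forward using a line trace that ignores enemies.
; Older teleport and preview code remains disconnected, so the Tick preview is never switched on here.
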(event `self.ReceiveBeginPlay`
  (set `self.MaxDash` 2.0)
  (set `self.MaxSpecialCooldown` 4.0)
  (set `self.SpecialCooldownTimer` 4.0))

(event `self.ReceiveTick`
  (params (DeltaSeconds :type "Float (single-precision)"))
  (bind _returnvalue (`self.K2_GetActorRotation`))
  (bind _aoerange (`self.AoERange`))
  (bind _teleportdistanceref (`self.TeleportDistanceRef`))
  (bind (_returnvalue_x _returnvalue_y) (`KismetMathLibrary.BreakVector` (`SceneComponent.K2_GetComponentLocation` (`self.CapsuleComponent`))))
  (bind (_returnvalue_x_2 _returnvalue_y_2 _returnvalue_z) (`KismetMathLibrary.BreakVector` (`SceneComponent.K2_GetComponentLocation` (`self.AoeTelegraphPoint`))))
  (bind _returnvalue_2 (`SceneComponent.K2_GetComponentLocation` (`self.CapsuleComponent`)))
  (bind _returnvalue_3 (* _aoerange -1.0))
  ;[1 1 1] This script allows the shaman to move around their aoe attack
  (`parent.ReceiveTick` DeltaSeconds)
  (`|ExecutionSequence`
    (:`then_0`
      (if (`self.IsAttacking?`)
        (`SceneComponent.K2_SetWorldLocation` (`self.AoeTelegraphPoint`) (`KismetMathLibrary.MakeVector` (`KismetMathLibrary.FClamp` (+ _returnvalue_x_2 (* (`self.GetInputAxisValue`) 30.0)) (+ _returnvalue_x _returnvalue_3) (+ _returnvalue_x _aoerange)) (`KismetMathLibrary.FClamp` (+ _returnvalue_y_2 (* (`self.GetInputAxisValue`) 30.0)) (+ _returnvalue_y _returnvalue_3) (+ _returnvalue_y _aoerange)) _returnvalue_z) false false)
        (else
          (`SceneComponent.K2_SetWorldLocation` (`self.AoeTelegraphPoint`) (`SceneComponent.K2_GetComponentLocation` (`self.AoeTelegraphPointOrigin`)) false false))))
    (:`then_1`
      (if (`self.TeleportHeld?`)
        (bind _outactors (`GameplayStatics.GetAllActorsOfClass` "/Game/EPOC_BP/Enemy/BP_Enemy.BP_Enemy_C"))
        (bind _outhit (`KismetSystemLibrary.LineTraceSingle` _returnvalue_2 (+ _returnvalue_2 (* (`KismetMathLibrary.GetForwardVector` (`self.K2_GetActorRotation`)) (`self.DashDistance`))) "TraceTypeQuery1" false _outactors "ForDuration"))
        (bind (_bblockinghit _binitialoverlap _time _distance _location _impactpoint _normal _impactnormal _physmat _hitactor _hitcomponent _hitbonename _bonename _hititem _elementindex _faceindex _tracestart _traceend) (`GameplayStatics.BreakHitResult` _outhit))
        (if _bblockinghit
          (bind _returnvalue_4 (`self.K2_TeleportTo` _teleportdistanceref _location _returnvalue))
          (if (not _returnvalue_4)
            (`self.K2_TeleportTo` _teleportdistanceref _tracestart _returnvalue))
          (else
            (`self.K2_TeleportTo` _teleportdistanceref _traceend (`self.K2_GetActorRotation`))))
        (elif (not (== (`self.TeleportDistanceRef`) null))
          (`self.K2_DestroyActor` (`self.TeleportDistanceRef`)))))))

(event `InputAction|SpecialAttack`
  (params (Key :type "Key Structure"))
  (bind _mesh (`self.Mesh`))
  (bind (_returnvalue_roll _returnvalue_pitch _returnvalue_yaw) (`KismetMathLibrary.BreakRotator` (`KismetMathLibrary.MakeRotFromX` (`self.GetActorForwardVector`))))
  (:`Pressed`
    (if (`self.IsAttacking?`)
      _
      (elif (>= (`self.SpecialCooldownTimer`) (`self.MaxSpecialCooldown`))
        (set `self.IsSpecialAttacking?` true)
        (`|SpawnActorFromClass` "/Game/EPOC_BP/EPOC_CONTENT/Blueprints/PlayerBlueprints/ShamanPlayer/BP_Bolt.BP_Bolt_C" (`self.GetTransform` self) "Undefined" "OverrideRootScale" null self null)
        (`NiagaraFunctionLibrary.SpawnSystemAttached` "/Game/VFX_/VFX_Shaman/VFX_Shaman_Skill/VFX_DarkLighting/VFX__Darklighting.VFX__Darklighting" _mesh "None" (`SceneComponent.K2_GetComponentLocation` _mesh) (`KismetMathLibrary.MakeRotator` 0.0 0.0 _returnvalue_yaw) "KeepWorldPosition" true)
        (set `self.SpecialCooldownTimer` 0.0)
        (`KismetSystemLibrary.K2_SetTimer` null "SpecialCooldown" 0.01 true))))
  (:`Released`
    (if (`self.IsSpecialAttacking?`)
      (set `self.IsSpecialAttacking?` false))))

(event `InputAction|BasicAttack`
  (params (Key :type "Key Structure"))
  (bind _aoetelegraphpoint (`self.AoeTelegraphPoint`))
  (bind (_returnvalue_x _returnvalue_y _returnvalue_z) (`KismetMathLibrary.BreakVector` (`SceneComponent.K2_GetComponentLocation` _aoetelegraphpoint)))
  (bind (_returnvalue_location _returnvalue_rotation) (`KismetMathLibrary.BreakTransform` (`SceneComponent.K2_GetComponentToWorld` (`self.AoeTelegraphPoint`))))
  (:`Pressed`
    (set `self.isCharging` true)
    (set `self.IsAttacking?` true)
    (bind _returnvalue (`|SpawnActorFromClass` "/Game/EPOC_BP/VFX_/VFX_Decal/VFX_Actor_CircleSkill.VFX_Actor_CircleSkill_C" (`KismetMathLibrary.MakeTransform` (`KismetMathLibrary.MakeVector` (+ _returnvalue_x 0.0) (+ _returnvalue_y 0.0) _returnvalue_z) (`SceneComponent.K2_GetComponentRotation` _aoetelegraphpoint) (2.0 2.0 2.0)) "Undefined" "OverrideRootScale" null null))
    (bind _output_get (set `self.CircleSkillRef` _returnvalue))
    (`self.K2_AttachToComponent` _output_get (`self.AoeTelegraphPoint`) "None" "KeepWorld" "KeepWorld" "KeepWorld" true)
    (bind _returnvalue_2 (`KismetSystemLibrary.K2_SetTimer` null "BombChargeTime" 0.01 true)))
  (:`Released`
    (set `self.isCharging` false)
    (`KismetSystemLibrary.K2_ClearAndInvalidateTimerHandle` _returnvalue_2)
    (if (>= (`self.BombCharge`) 0.5)
      (`|SpawnActorFromClass` "/Game/EPOC_BP/EPOC_CONTENT/Blueprints/PlayerBlueprints/ShamanPlayer/BP_Bomb.BP_Bomb_C" (`KismetMathLibrary.MakeTransform` _returnvalue_location _returnvalue_rotation (1.5 1.5 1.5)) "Undefined" "OverrideRootScale" null self 0.0 7.0 0.0 null))
    (set `self.BombCharge` 0.0)
    (`self.K2_DestroyActor` (`self.CircleSkillRef`))
    (set `self.IsAttacking?` false)))

(event `InputAction|Jump`
  (params (Key :type "Key Structure"))
  (bind _returnvalue (`self.K2_GetActorRotation`))
  (bind _dashfx_location (`self.DashFX_Location`))
  (bind (_returnvalue_roll _returnvalue_pitch _returnvalue_yaw) (`KismetMathLibrary.BreakRotator` (`KismetMathLibrary.MakeRotFromX` (`self.GetActorForwardVector`))))
  (bind _returnvalue_2 (`SceneComponent.K2_GetComponentLocation` (`self.CapsuleComponent`)))
  ;[1 1 1] Shaman's unique teleport which overrides the parent dash
  (:`Pressed`
    (set `self.TeleportHeld?` false)
    (if (>= (`self.dashTimer`) 1.5)
      (bind _outactors (`GameplayStatics.GetAllActorsOfClass` "/Game/EPOC_BP/Enemy/BP_Enemy.BP_Enemy_C"))
      (bind _outhit (`KismetSystemLibrary.LineTraceSingle` _returnvalue_2 (+ _returnvalue_2 (* (`KismetMathLibrary.GetForwardVector` (`self.K2_GetActorRotation`)) (`self.DashDistance`))) "TraceTypeQuery1" false _outactors))
      (bind (_bblockinghit _binitialoverlap _time _distance _location _impactpoint _normal _impactnormal _physmat _hitactor _hitcomponent _hitbonename _bonename _hititem _elementindex _faceindex _tracestart _traceend) (`GameplayStatics.BreakHitResult` _outhit))
      (if _bblockinghit
        (bind _returnvalue_3 (`self.K2_TeleportTo` _traceend _returnvalue))
        (if (not _returnvalue_3)
          (`self.K2_TeleportTo` _location _returnvalue)
          (set `self.dashTimer` 0.0 :!label _label)
          (bind _returnvalue_4 (`NiagaraFunctionLibrary.SpawnSystemAttached` "/Game/VFX_/VFX_Shaman/VFX_Shaman_Dash/VFX__Shaman_Dash_NS.VFX__Shaman_Dash_NS" _dashfx_location "None" (`SceneComponent.K2_GetComponentLocation` _dashfx_location) (`KismetMathLibrary.MakeRotator` 0.0 0.0 _returnvalue_yaw) "KeepWorldPosition"))
          (set `self.DashVFX` _returnvalue_4)
          (`Timeline|Timeline_0_0` :!via `PlayFromStart`
            (:`Finished`
              (`ActorComponent.Deactivate` (`self.DashVFX`)))))
        (else
          (`self.K2_TeleportTo` _traceend (`self.K2_GetActorRotation`))
          (goto _label))))))

(fn `BombChargeTime`
  (set `self.BombCharge` (`KismetMathLibrary.FClamp` (+ (`self.BombCharge`) 0.01) 0.0 3.0)))

(fn `SpawnAOE`
  (params (Location :type "Vector Structure") (Radius :type "Float (double-precision)") (RequireLOS :type Boolean) (AOE_Instigator :type "Actor Object Reference") (DrawDebugDuration :type "Float (double-precision)") (DebugColor :type "LinearColor Structure"))
  (if (> (`local.DrawDebugDuration`) 0.0)
    (`KismetSystemLibrary.DrawDebugSphere` Location Radius 16 DebugColor DrawDebugDuration 2.0)
    (bind _outactors (`KismetSystemLibrary.SphereOverlapActors` Location Radius (`|MakeArray` "ObjectTypeQuery3" :!type "EObjectTypeQuery Enum") "/Game/EPOC_BP/Enemy/BP_Enemy.BP_Enemy_C" (`|MakeArray` AOE_Instigator)))
    (for _array_element _outactors
      (bind _output_get (set `self.CurrentActor` _array_element))
      (`GameplayStatics.ApplyDamage` _output_get 1.0))))

(fn `SpecialCooldown`
  (set `self.SpecialCooldownTimer` (`KismetMathLibrary.FClamp` (+ (`self.SpecialCooldownTimer`) 0.01) 0.0 (`self.MaxSpecialCooldown`))))

(fn `UserConstructionScript`
  (`parent.UserConstructionScript`))