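; BP_ArrowRain is a short-lived area damage skill actor that plays an arrow rain Niagara effect on its BombCollision and destroys itself after a few seconds.
; Each tick it queries that collision for BP_Player pawns, ignoring BombCreator.
; The first actor hit takes InitDamage and sets the shared BombSpawned flag, so every later hit deals DoTDamage per frame, unscaled by delta time.
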(event `self.ReceiveBeginPlay`
  (bind _bombcollision (`self.BombCollision`))
  (bind (_returnvalue_roll _returnvalue_pitch _returnvalue_yaw) (`KismetMathLibrary.BreakRotator` (`KismetMathLibrary.MakeRotFromX` (`self.GetActorForwardVector`))))
  (`NiagaraFunctionLibrary.SpawnSystemAttached` "/Game/VFX_/VFX_Enemy/VFX_Enemy_Skill_ArrowRain/VFX_Enemy_Skill_ArrowRain_NS_ParabolaRain.VFX_Enemy_Skill_ArrowRain_NS_ParabolaRain" _bombcollision "None" (`SceneComponent.K2_GetComponentLocation` _bombcollision) (`KismetMathLibrary.MakeRotator` 0.0 0.0 _returnvalue_yaw) "KeepWorldPosition" true)
  (`KismetSystemLibrary.Delay` 3.0)
  (`self.K2_DestroyActor`))

(event `self.ReceiveTick`
  (params (DeltaSeconds :type "Float (single-precision)"))
  (bind _bombcollision (`self.BombCollision`))
  (bind _outactors (`KismetSystemLibrary.ComponentOverlapActors` _bombcollision (`SceneComponent.K2_GetComponentToWorld` _bombcollision) (`|MakeArray` "ObjectTypeQuery3" :!type "EObjectTypeQuery Enum") "/Game/EPOC_BP/EPOC_CONTENT/Blueprints/PlayerBlueprints/BP_Player.BP_Player_C" (`|MakeArray` (`self.BombCreator`))))
  (for _array_element _outactors
    (if (`self.BombSpawned?`)
      (`GameplayStatics.ApplyDamage` _array_element (`self.DoTDamage`))
      (cast `/Game/EPOC_BP/Enemy/BP_Enemy` _array_element)
      (else
        (`GameplayStatics.ApplyDamage` _array_element (`self.InitDamage`))
        (set `self.BombSpawned?` true)))))

(fn `UserConstructionScript`
  (set `self.BombSpawned?` false))