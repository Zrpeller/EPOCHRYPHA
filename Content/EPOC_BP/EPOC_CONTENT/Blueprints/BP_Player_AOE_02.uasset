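; BP_Player_AOE_02 is a player Blueprint for a press-and-release area attack on the BasicAttack input.
; Pressing spawns a circle VFX actor attached to AoeTelegraphPoint as a telegraph; releasing calls SpawnAOE there, then destroys it.
; SpawnAOE draws a debug sphere, damages overlapping Enemy pawns and prints their names.
; All of this runs only when debug duration is positive, and RequireLOS is unused.
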(event `InputAction|BasicAttack`
  (params (Key :type "Key Structure"))
  (bind _aoetelegraphpoint (`self.AoeTelegraphPoint`))
  (:`Pressed`
    (set `self.IsAttacking?` true)
    (bind _returnvalue (`|SpawnActorFromClass` "/Game/EPOC_BP/VFX_/VFX_Decal/VFX_Actor_CircleSkill.VFX_Actor_CircleSkill_C" (`KismetMathLibrary.MakeTransform` (`SceneComponent.K2_GetComponentLocation` _aoetelegraphpoint) (`SceneComponent.K2_GetComponentRotation` _aoetelegraphpoint)) "Undefined" "OverrideRootScale" null null))
    (bind _output_get (set `self.CircleSkillRef` _returnvalue))
    (`self.K2_AttachToComponent` _output_get (`self.AoeTelegraphPoint`) "None" "KeepWorld" "KeepWorld" "KeepWorld" true))
  (:`Released`
    (set `self.IsAttacking?` false)
    (`self.SpawnAOE` (`SceneComponent.K2_GetComponentLocation` (`self.AoeTelegraphPoint`)) 350.0 false self 2.5 (struct :`G` 0.075142 :`B` 1.0 :`A` 1.0))
    (`self.K2_DestroyActor` (`self.CircleSkillRef`))))

(fn `SpawnAOE`
  (params (Location :type "Vector Structure") (Radius :type "Float (double-precision)") (RequireLOS :type Boolean) (AOE_Instigator :type "Actor Object Reference") (DrawDebugDuration :type "Float (double-precision)") (DebugColor :type "LinearColor Structure"))
  (if (> (`local.DrawDebugDuration`) 0.0)
    (`KismetSystemLibrary.DrawDebugSphere` Location Radius 16 DebugColor DrawDebugDuration 2.0)
    (bind _outactors (`KismetSystemLibrary.SphereOverlapActors` Location Radius (`|MakeArray` "ObjectTypeQuery3" :!type "EObjectTypeQuery Enum") "/Game/EPOC_BP/Enemy/Enemy.Enemy_C" (`|MakeArray` AOE_Instigator)))
    (for _array_element _outactors
      (bind _output_get (set `self.CurrentActor` _array_element))
      (`GameplayStatics.ApplyDamage` _output_get 10.0)
      (`KismetSystemLibrary.PrintString` (`KismetSystemLibrary.GetDisplayName` _output_get)))))

(fn `UserConstructionScript`
  (`parent.UserConstructionScript`))