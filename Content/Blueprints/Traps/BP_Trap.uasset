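; Trap actor that damages actors tagged Player when they begin overlapping its Box component.
; The overlap applies a single hit of damage and prints the result, without destroying the trap.
; A poison-over-time chain using the local ForLoopWithDelay macro, which spaces iterations with a Delay, and the DestroyActor calls are unwired and never run.
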(event `self.Box.OnComponentBeginOverlap`
  (params (OverlappedComponent :type "PrimitiveComponent Object Reference") (OtherActor :type "Actor Object Reference") (OtherComp :type "PrimitiveComponent Object Reference") (OtherBodyIndex :type Integer) (bFromSweep :type Boolean) (SweepResult :type "HitResult Structure (by ref)"))
  ;[1 1 1] Damage then destroy
  (if (`self.ActorHasTag` OtherActor "Player")
    (bind _returnvalue (`GameplayStatics.ApplyDamage` OtherActor 1.0))
    (`KismetSystemLibrary.PrintString` (`KismetStringLibrary.Conv_DoubleToString` _returnvalue))))

(fn `UserConstructionScript`)