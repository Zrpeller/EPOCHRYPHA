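; BP_Trap_Continuous is a trap that repeatedly damages players standing inside its Box volume.
; The first Box overlap by any actor starts a half-second Delay loop that applies a small fixed damage to every overlapping BP_Player.
; End overlap is empty, so the loop never stops and relies on the overlap query to spare players who leave.
; The TouchingTrap-gated loop and For Loop With Delay macro are unused.
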(event `self.Box.OnComponentBeginOverlap`
  (params (OverlappedComponent :type "PrimitiveComponent Object Reference") (OtherActor :type "Actor Object Reference") (OtherComp :type "PrimitiveComponent Object Reference") (OtherBodyIndex :type Integer) (bFromSweep :type Boolean) (SweepResult :type "HitResult Structure (by ref)"))
  ;[1 1 1] Damage then destroy
  (if true
    (set `self.TouchingTrap?` true)
    (`self.DamagePlayers` :!label _label)
    (`KismetSystemLibrary.Delay` 0.5)
    (goto _label)))

(event `self.Box.OnComponentEndOverlap`
  (params (OverlappedComponent :type "PrimitiveComponent Object Reference") (OtherActor :type "Actor Object Reference") (OtherComp :type "PrimitiveComponent Object Reference") (OtherBodyIndex :type Integer))
  ;[1 1 1] Stop damaging player
)

(event `DamagePlayers`
  (for _array_element (`PrimitiveComponent.GetOverlappingActors` (`self.Box`) "/Game/EPOC_BP/EPOC_CONTENT/Blueprints/PlayerBlueprints/BP_Player.BP_Player_C")
    (`GameplayStatics.ApplyDamage` _array_element 0.6)))

(fn `UserConstructionScript`
  (`parent.UserConstructionScript`))